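; BP_Task is an interactable task station that launches a minigame for one of two local players.
; Its sphere overlap shows or hides a per-player prompt widget, shown only while the task is active and unoccupied.
; Interact claims the station, removes both prompts and, if active, starts the minigame selected by MinigameID, passing the player controller and itself.
; A temporary BeginPlay hook activates Refuel and Motor Winding tasks.
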(event `self.Sphere.OnComponentBeginOverlap`
  (params (OverlappedComponent :type "PrimitiveComponent Object Reference") (OtherActor :type "Actor Object Reference") (OtherComp :type "PrimitiveComponent Object Reference") (OtherBodyIndex :type Integer) (bFromSweep :type Boolean) (SweepResult :type "HitResult Structure (by ref)"))
  ;[1 0.7294 0 0.502] Visibility of Interaction Widget
  ;; adds to view when player enters the collider
  (bind _returnvalue (`self.DoesHaveInteractingPlayer`))
  (if _returnvalue
    _
    (elif (`self.ActorHasTag` OtherActor "Player")
      (bind _returnvalue_2 (`self.GetActiveState`))
      (if _returnvalue_2
        (bind _asplayer_controller (cast `PlayerController` (`self.GetInstigatorController` OtherActor)))
        (if (== (`GameplayStatics.GetPlayerControllerID` _asplayer_controller) 0)
          (`UserWidget.AddToViewport` (`self.InteractionWidgetP1`) 0)
          (else
            (`UserWidget.AddToViewport` (`self.InteractionWidgetP2`) 0)))))))

(event `self.Sphere.OnComponentEndOverlap`
  (params (OverlappedComponent :type "PrimitiveComponent Object Reference") (OtherActor :type "Actor Object Reference") (OtherComp :type "PrimitiveComponent Object Reference") (OtherBodyIndex :type Integer))
  ;[1 0.7294 0 0.502] Visibility of Interaction Widget
  ;; removes from view when player leaves the collider
  (if (`self.ActorHasTag` OtherActor "Player")
    (bind _asplayer_controller (cast `PlayerController` (`self.GetInstigatorController` OtherActor)))
    (if (== (`GameplayStatics.GetPlayerControllerID` _asplayer_controller) 0)
      (`Widget.RemoveFromParent` (`self.InteractionWidgetP1`))
      (else
        (`Widget.RemoveFromParent` (`self.InteractionWidgetP2`))))))

(event `Interact`
  (params (InteractingPlayer :type "PlayerController Object Reference"))
  ;[0 0.5137 1 0.502] Selection of Minigame
  (bind _returnvalue (`self.DoesHaveInteractingPlayer`))
  (if (not _returnvalue)
    (set `self.Interacting Player` InteractingPlayer)
    (if (`KismetSystemLibrary.IsValid` InteractingPlayer)
      (`self.SetHasInteractingPlayer` true)
      (`Widget.RemoveFromParent` (`self.InteractionWidgetP2`))
      (`Widget.RemoveFromParent` (`self.InteractionWidgetP1`))
      (switch `int` (`self.MinigameID`)
        (:`0`
          ;; Minigame1
          (bind _asbp_minigame (cast `/Game/Code/Blueprints/Tasks/Minigames/BP_Minigame` (`self.Minigame`)))
          (bind _returnvalue_2 (`self.GetActiveState`))
          (if _returnvalue_2
            (`/Game/Code/Blueprints/Tasks/Minigames/BP_Minigame.Event MinigameBegin` _asbp_minigame (`self.Interacting Player`) self)))
        (:`1`
          ;; Minigame3
          (bind _asbp_minigame_3 (cast `/Game/Code/Blueprints/Tasks/Minigames/BP_Minigame3` (`self.Minigame`)))
          (bind _returnvalue_3 (`self.GetActiveState`))
          (if _returnvalue_3
            (`/Game/Code/Blueprints/Tasks/Minigames/BP_Minigame3.Event MinigameBegin` _asbp_minigame_3 (`self.Interacting Player`) self)))
        (:`2`
          ;; Mingame4
          (bind _asbp_minigame_4 (cast `/Game/Code/Blueprints/Tasks/Minigames/BP_Minigame4` (`self.Minigame`)))
          (bind _returnvalue_4 (`self.GetActiveState`))
          (if _returnvalue_4
            (`/Game/Code/Blueprints/Tasks/Minigames/BP_Minigame4.Event MinigameBegin` _asbp_minigame_4 (`self.Interacting Player`) self)))
        (:`3`
          ;; Mingame5
          (bind _asbp_minigame_5 (cast `/Game/Code/Blueprints/Tasks/Minigames/BP_Minigame5` (`self.Minigame`)))
          (bind _returnvalue_5 (`self.GetActiveState`))
          (if _returnvalue_5
            (`/Game/Code/Blueprints/Tasks/Minigames/BP_Minigame5.Event MinigameBegin` _asbp_minigame_5 (`self.Interacting Player`) self)))))))

(event `self.ReceiveBeginPlay`
  ;[0 0.5137 1 0.502] Selection of Minigame
  ;;[1 0.8661 0.1264 0.5] Temp, REMOVE LATER!!!
  (bind _returnvalue (`self.GetTaskType`))
  (switch `|SwitchEnum` _returnvalue
    (:`Refuel`
      _)
    (:`MotorWinding`
      _))
  (`self.SetActive` true))

(fn `UserConstructionScript`)