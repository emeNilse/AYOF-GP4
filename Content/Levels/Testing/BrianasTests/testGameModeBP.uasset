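; Test game mode that plays dialogue at the start and end of seasons and advances to the next season.
; BeginPlay triggers StartSeason, while EndSeason plays its dialogue event and then immediately calls LoadNextSeason.
; Both season events build the dialogue key from the CurrentSeason enum name plus a "Start" or "End" suffix and pass it to SeasonsDialogueComponent.
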(event `self.ReceiveBeginPlay`
  (`self.StartSeason`))

(event `self.EndSeason`
  (`DialogueEventComponent.StartDialogueEvent` (`self.SeasonsDialogueComponent`) (`KismetStringLibrary.Conv_StringToName` (`KismetStringLibrary.Concat_StrStr` (`|GetEnumeratorNameAsString` (`self.CurrentSeason`)) "End")) false)
  (`self.LoadNextSeason` true))

(event `self.StartSeason`
  (`DialogueEventComponent.StartDialogueEvent` (`self.SeasonsDialogueComponent`) (`KismetStringLibrary.Conv_StringToName` (`KismetStringLibrary.Concat_StrStr` (`|GetEnumeratorNameAsString` (`self.CurrentSeason`)) "Start")) false))

(fn `UserConstructionScript`)