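; Player controller that creates the local player's HUD and handles the inventory input.
; On BeginPlay it adds W_PlayerHUD to the viewport, then collapses it and sets a main-menu flag if the CameraActor it finds is tagged MenuCamera.
; The open-inventory input toggles the HUD inventory unless in the main menu or possessing a cooking station.
; LookAt and SelectFromInventory are empty stubs.
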(event `self.ReceiveBeginPlay`
  (if (`self.IsLocalPlayerController`)
    (bind _returnvalue (`|CreateWidget` "/Game/Code/UI/UI_Inventory/W_PlayerHUD.W_PlayerHUD_C"))
    (bind _output_get (set `self.HUD` _returnvalue))
    (`UserWidget.AddToViewport` _output_get 0)
    (bind _returnvalue_2 (`GameplayStatics.GetActorOfClass` "/Script/Engine.CameraActor"))
    (if (`self.ActorHasTag` _returnvalue_2 "MenuCamera")
      (`Widget.SetVisibility` (`self.HUD`) "Collapsed")
      (set `self.IsInMainMenu` true))))

(event `EnhancedInput|/Game/Code/Input/Actions/IA_OpenInventory`
  (params (ActionValue :type Boolean) (ElapsedSeconds :type "Float (double-precision)") (TriggeredSeconds :type "Float (double-precision)") (InputAction :type "InputAction Object Reference" :default "/Game/Code/Input/Actions/IA_OpenInventory.IA_OpenInventory"))
  (:`Completed`
    (if (not (`self.IsInMainMenu`))
      (bind _returnvalue (`self.GetIsPossessingCookingStation`))
      (if (not _returnvalue)
        (`/Game/Code/UI/UI_Inventory/W_PlayerHUD.TogglePlayerInventory` (`self.HUD`))))))

(fn `LookAt`
  (returns (Message :type Text))
  (return ""))

(fn `SelectFromInventory`
  (return))

(fn `UserConstructionScript`)