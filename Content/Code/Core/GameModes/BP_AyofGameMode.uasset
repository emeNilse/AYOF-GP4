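; Game mode that runs one season of the game, from opening dialogue to loading the next season or the end menu.
; StartSeason enables player input and plays the season's start dialogue, using keys built from the season enum name.
; EndSeason disables input, plays the end dialogue and attempts the tagged final-dish sequence.
; Tick polls a load flag, waiting for dialogue to finish before advancing or, in the final season, ending the game.
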(event `self.ReceiveBeginPlay`
  (bind _asbp_game_instance (cast `/Game/Code/Core/BP_GameInstance` (`GameplayStatics.GetGameInstance`))
    (:`then`
      (`/Game/Code/Core/BP_GameInstance.StartSeason` _asbp_game_instance (`self.CurrentSeason`)))
    (:`CastFailed`
      _))
  (`self.StartSeason`))

(event `self.ReceiveTick`
  (params (DeltaSeconds :type "Float (single-precision)"))
  (if (and (`self.LoadNextLevelTriggered`) (not (`DialogueManagerComponent.IsDialoguePlaying` (`self.DialogueManager`))))
    (if (`self.IsFinalSeason`)
      (`/Engine/EditorBlueprintResources/StandardMacros.DoOnce` false
        (:`Completed`
          (`self.EndGame`)))
      (else
        (`self.LoadNextSeason` true)))))

(event `self.StartSeason`
  (bind _asbp_character (cast `/Game/Code/Player/BP_Character` (`GameplayStatics.GetPlayerCharacter` 0)))
  (`self.EnableInput` _asbp_character null)
  (`self.PlaySeasonDialogue` true)
  (`self.SeasonStarted` 0))

(event `self.EndSeason`
  (`self.DisablePlayerInput`)
  (`self.PlaySeasonDialogue` false)
  (bind _bcutscenestarted (`self.PlayCutscene` "FinalDishCut"))
  (if (not _bcutscenestarted)
    (set `self.LoadNextLevelTriggered` true)))

(event `self.EndGame`
  (`KismetSystemLibrary.Delay` 0.2)
  (`self.ShowEndGameMenu`))

(event `OnCutsceneFinished`
  ; Cutscene
)

(fn `OnCutsceneEnd`
  (set `self.LoadNextLevelTriggered` true))

(fn `PlayCutscene`
  (params (CutSceneTag :type Name :default "FinalDishCut"))
  (returns (bCutsceneStarted :type Boolean))
  ; Cutscene
  (bind _asmy_player_controller (cast `MyPlayerController` (`GameplayStatics.GetPlayerController` 0))
    (:`then`
      (bind _asbp_character (cast `/Game/Code/Player/BP_Character` (`MyPlayerController.CharacterPawn` _asmy_player_controller))
        (:`then`
          (`/Game/Code/Player/BP_Character.HideCursor` _asbp_character)
          (bind _outactors (`GameplayStatics.GetAllActorsOfClassWithTag` "/Script/LevelSequence.LevelSequenceActor" (`local.CutSceneTag`)))
          (bind _sequenceplayer (`LevelSequenceActor.SequencePlayer` (`|GetArrayItem` _outactors)))
          (`MovieSceneSequencePlayer.Play` _sequenceplayer)
          (add `MovieSceneSequencePlayer.OnFinished` _sequenceplayer (`|CreateDelegate` :!event `OnCutsceneEnd`))
          (return true))
        (:`CastFailed`
          _)))
    (:`CastFailed`
      _))
  (return false))

(fn `PlaySeasonDialogue`
  (params (bIsStart :type Boolean :default true))
  (bind _returnvalue (`KismetStringLibrary.Concat_StrStr` (`|GetEnumeratorNameAsString` (`self.CurrentSeason`)) "Start"))
  (if bIsStart
    (`KismetSystemLibrary.PrintString` _returnvalue)
    ; season start dialogue
    (`DialogueEventComponent.StartDialogueEvent` (`self.SeasonsDialogueComponent`) (`KismetStringLibrary.Conv_StringToName` _returnvalue) false)
    (else
      ; Season end dialogue
      (`DialogueEventComponent.StartDialogueEvent` (`self.SeasonsDialogueComponent`) (`KismetStringLibrary.Conv_StringToName` (`KismetStringLibrary.Concat_StrStr` (`|GetEnumeratorNameAsString` (`self.CurrentSeason`)) "End")) false))))

(fn `ShowEndGameMenu`
  (bind _boutsuccess (`LevelStreamingDynamic.LoadLevelInstanceBySoftObjectPtr` "/Game/Levels/Official/EndMenu.EndMenu" (0.0 0.0 0.0) (struct) "" null))
  (`WidgetLayoutLibrary.RemoveAllWidgets`)
  (bind _returnvalue (`|CreateWidget` "/Game/Code/UI/Menus/WB_LoadingScreen.WB_LoadingScreen_C" (`GameplayStatics.GetPlayerController` 0)))
  (`UserWidget.AddToViewport` _returnvalue 0)
  (if _boutsuccess
    (`GameplayStatics.OpenLevelBySoftObjectPtr` "/Game/Levels/Official/EndMenu.EndMenu")))

(fn `UserConstructionScript`)