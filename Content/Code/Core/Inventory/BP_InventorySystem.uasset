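; BP_InventorySystem is an inventory component that stores item slots, handles player interaction and checks held items against crafting recipes.
; A Tick sphere trace from the camera sets LookAtActor, which the interact input sends to a server event.
; Adding fills stacks before empty slots using data-table limits, while transfers swap differing slots between inventories.
; Removal can spawn dropped items, and removals and transfers broadcast UI updates through a multicast event.
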(event `self.ReceiveBeginPlay`
  (`KismetArrayLibrary.Array_Resize` (`self.Content`) (`self.InventorySize`))
  (set `self.RecipesList` "/Game/Code/Core/Inventory/BT_Recipes.BT_Recipes"))

(event `self.ReceiveTick`
  (params (DeltaSeconds :type "Float (single-precision)"))
  ;[1 0.8294 0 0.5] In prossess of being phased out
  (`self.InteractionTrace`))

(event `EnhancedInput|/Game/Code/Input/Actions/IA_Interact`
  (params (ActionValue :type Boolean) (ElapsedSeconds :type "Float (double-precision)") (TriggeredSeconds :type "Float (double-precision)") (InputAction :type "InputAction Object Reference" :default "/Game/Code/Input/Actions/IA_Interact.IA_Interact")))

(event `EnhancedInput|/Game/Code/Input/Actions/IA_InventoryInteract`
  (params (ActionValue :type Boolean) (ElapsedSeconds :type "Float (double-precision)") (TriggeredSeconds :type "Float (double-precision)") (InputAction :type "InputAction Object Reference" :default "/Game/Code/Input/Actions/IA_InventoryInteract.IA_InventoryInteract"))
  ; Interacting with item
  ;; If interacting with a actor or pawn with ItemDataComponent or InventorySystem run logic
  (:`Triggered`
    (bind _lookatactor (`self.LookAtActor`)
      (:`then`
        (`self.Server_Interact` _lookatactor))
      (:`else`))))

(event `Server_Interact`
  (params (Target :type "Actor Object Reference"))
  (bind _returnvalue (`Actor.GetComponentByClass` Target "/Game/Code/Core/Inventory/BP_ItemDataComponent.BP_ItemDataComponent_C"))
  (bind _returnvalue_2 (`Pawn.GetController` (cast `/Game/Code/Player/BP_Character` (`self.GetOwner`) :!pure true)))
  ; Interacting with item
  (`/Engine/EditorBlueprintResources/StandardMacros.IsValid` _returnvalue
    (:`Is Valid`
      ;; Interface Function IInterface
      (message `/Game/Code/Core/Inventory/IInteractInterface.InteractWith` _returnvalue (cast `/Game/Code/Player/BP_Character` (`self.GetOwner`) :!pure true)))
    (:`Is Not Valid`
      (`Actor.SetOwner` Target _returnvalue_2)
      (`self.OnLocalInteract` Target _returnvalue_2))))

(event `OnLocalInteract`
  (params (TargetActor :type "Actor Object Reference") (Interactor :type "Actor Object Reference"))
  ; Interacting with item
  (message `/Game/Code/Core/Inventory/IInteractInterface.InteractWith` TargetActor (cast `/Game/Code/Player/BP_Character` Interactor :!pure true)))

(event `MC_Update`
  ; Update the inventory
  (`self.OnInventoryUpdated`))

(event `SERVER_TransferSlots`
  (params (SourceIndex :type Integer) (SourceInventory :type "/Game/Code/Core/Inventory/BP_InventorySystem Object Reference") (DestinationIndex :type Integer))
  ; Gets called OnDrop event in W_Inventory slots. Function transfer item ID from one slot to another
  (`self.TransferSlots` SourceIndex SourceInventory DestinationIndex))

(event `ServerRemove`
  (params (Index :type Integer) (RemoveCompletely :type Boolean))
  ; Removes item from provided Inventory and inventory slot index (Example usage in W_UIActionMenu)
  (`self.RemoveFromInventory` Index RemoveCompletely))

(event `ServerDropItem`
  (params (ItemID :type Name) (Quantity :type Integer))
  ; Spawns Item in world (Not used anywhere ATM) Gets called in the Remove From Inventory function
  (for _ (range Quantity)
    (`|SpawnActorFromClass` (`.ItemClass` (break `ItemAssetData` (`.ItemAssetData` (break `ItemDataStruct` (`self.GetItemData` ItemID))))) (`KismetMathLibrary.MakeTransform` (`self.GetDropLocation`)) "Undefined" "MultiplyWithRoot" null null)))

(fn `AddToInventory`
  (params (ItemID :type Name) (Quantity :type Integer))
  (returns (Success :type Boolean) (QuantityRemaining :type Integer))
  (locals (LocalQuantityRemaining :type Integer :default 0) (LocalHasFailed :type Boolean))
  (set `local.LocalQuantityRemaining` Quantity)
  (while (and (> (`local.LocalQuantityRemaining`) 0) (not (`local.LocalHasFailed`)))
    ; Add to stack if item stackable and is not max stack
    (bind (_index _foundslot) (`self.FindSlot` (`local.ItemID`)))
    (if _foundslot
      (`KismetSystemLibrary.PrintText` "Found Stack")
      (`self.AddToStack` _index 1)
      (`/Engine/EditorBlueprintResources/StandardMacros.DecrementInt` (`local.LocalQuantityRemaining`))
      (else
        ; Adds item to empty slot
        (if (`self.AnyEmptySlotsAvalible`)
          (`KismetSystemLibrary.PrintString` "Found Empty slot")
          (bind _success (`self.CreateStack` (`local.ItemID`) 1))
          (if _success
            (`/Engine/EditorBlueprintResources/StandardMacros.DecrementInt` (`local.LocalQuantityRemaining`))
            (else
              ;; If we dont find an avalible stack or inventory has no empty slots return unsuccessful atempt to add item
              (set `local.LocalHasFailed` true)))
          (else
            (set `local.LocalHasFailed` true))))))
  ; If item successfuly added to inventory return success
  (return (not (`local.LocalHasFailed`)) (`local.LocalQuantityRemaining`)))

(fn `AddToStack`
  (params (Index :type Integer) (Quantity :type Integer))
  (bind (_output_itemid _output_quantity) (break `/Game/Code/Core/Inventory/FSlotStruct` (`|GetArrayItem` (`self.Content`) Index)))
  ; Gets the item ID added to inventory and sets matching ID already in inventory's quantity to +1
  (`KismetArrayLibrary.Array_Set` (`self.Content`) Index (make `/Game/Code/Core/Inventory/FSlotStruct` _output_itemid (+ _output_quantity (`local.Quantity`)))))

(fn `AnyEmptySlotsAvalible`
  (returns (HasEmptySlot :type Boolean) (EmptyIndex :type Integer))
  (for (_array_element _array_index) (`self.Content`)
    (bind (_itemid _quantity) (break `/Game/Code/Core/Inventory/FSlotStruct` _array_element))
    ; Check if a slots quantity is 0 and therefor empty
    (`KismetSystemLibrary.PrintText` (`KismetTextLibrary.Conv_IntToText` _quantity))
    (if (== _quantity 0)
      (return true _array_index)))
  (return false -1))

(fn `CheckIngredients`
  (returns (RecipeFound :type Boolean) (SpawnItem :type "Actor Class Reference"))
  (bind _outrownames (`DataTableFunctionLibrary.GetDataTableRowNames` "/Game/Code/Core/Inventory/BT_Recipes.BT_Recipes"))
  (for _array_element _outrownames
    (bind _returnvalue (`|GetDataTableRow` "/Game/Code/Core/Inventory/BT_Recipes.BT_Recipes" _array_element)
      (:`then`
        (bind (_recipe_ingredients _recipe_result) (break `Recipe` (break `/Game/Code/Core/Inventory/FSlot_Recipe_Struct` _returnvalue)))
        (for _array_element_2 _recipe_ingredients
          (set `self.bFound` false)
          (for _array_element_3 (`self.Content`)
            (if (== (`.ItemID_2_9A35EB514A7E0F49F31B1696D16693F0` (break `/Game/Code/Core/Inventory/FSlotStruct` _array_element_3)) (`.ID` (break `ItemDataStruct` _array_element_2)))
              (set `self.bFound` true)
              (break)))
          (if (not (`self.bFound`))
            (break)))
        (if (`self.bFound`)
          (return true (`.ItemClass` (break `ItemAssetData` (`.ItemAssetData` (break `ItemDataStruct` _recipe_result)))))))))
  (return false null))

(fn `CreateStack`
  (params (ItemID :type Name) (Quantity :type Integer))
  (returns (Success :type Boolean))
  (bind (_hasemptyslot _emptyindex) (`self.AnyEmptySlotsAvalible`))
  ; Fills empty slot found with Item
  (if _hasemptyslot
    (`KismetArrayLibrary.Array_Set` (`self.Content`) _emptyindex (make `/Game/Code/Core/Inventory/FSlotStruct` (`local.ItemID`) (`local.Quantity`)))
    (return true)
    (else
      (return false))))

(fn `FindSlot`
  (params (ItemID :type Name))
  (returns (Index :type Integer) (FoundSlot :type Boolean))
  (bind _itemid (`local.ItemID`))
  (bind (_max_stack_size _is_stackable) (`self.GetMaxStackSize` _itemid))
  ; Loops through Inventory items and checks if item is stackable and if it has reached its max stack
  (for (_array_element _array_index) (`self.Content`)
    (bind (_itemid_2 _quantity) (break `/Game/Code/Core/Inventory/FSlotStruct` _array_element))
    (if (== _itemid_2 _itemid)
      (if (and (< _quantity _max_stack_size) _is_stackable)
        (return _array_index true)
        (else
          (`KismetSystemLibrary.PrintString` "Max stack size reached")))))
  ; No room left
  (return -1 false))

(fn `GetDropLocation`
  (returns (Location :type "Vector Structure"))
  (bind _returnvalue (`Actor.K2_GetActorLocation` (`self.GetOwner`)))
  (bind _outhit (`KismetSystemLibrary.LineTraceSingle` _returnvalue (+ _returnvalue (0.0 0.0 0.0)) "TraceTypeQuery1"))
  (return (`.Location` (`GameplayStatics.BreakHitResult` _outhit))))

(fn `GetItemData`
  (params (ItemID :type Name))
  (returns (ItemData :type "ItemDataStruct Structure"))
  ; Gets a single ItemID from a slot and returns the row of matching ItemID
  (bind _returnvalue (`|GetDataTableRow` "/Game/Code/Core/Inventory/ItemData.ItemData" ItemID)
    (:`then`
      (return _returnvalue))))

(fn `GetMaxStackSize`
  (params (ItemID :type Name))
  (returns (`Max Stack Size` :type Integer) (`Is Stackable` :type Boolean))
  ; Returns an Items max stack and if its stackable
  (bind _returnvalue (`|GetDataTableRow` "/Game/Code/Core/Inventory/ItemData.ItemData" ItemID)
    (:`then`
      (bind (_maxstacksize _isstackable) (break `ItemNumericData` (`.ItemNumericData` (break `ItemDataStruct` _returnvalue))))
      (return _maxstacksize _isstackable))
    (:`RowNotFound`
      (return -1 false))))

(fn `GetSlotItem`
  (returns (ID :type Name) (`Item Type` :type "EItemType Enum") (`Item Quality` :type "EItemQuality Enum") (`Item Grade` :type "EItemGrade Enum") (`Valid Minigame` :type "EValidMinigame Enum") (`Item Asset Data` :type "ItemAssetData Structure"))
  ; Loop throu each slot element in the saved array and break out item data, then outputs some variables to use
  (for _array_element (`self.Content`)
    (bind _returnvalue (`|GetDataTableRow` "/Game/Code/Core/Inventory/ItemData.ItemData" (`.ItemID_2_9A35EB514A7E0F49F31B1696D16693F0` (break `/Game/Code/Core/Inventory/FSlotStruct` _array_element)))
      (:`then`
        (bind (_id _itemtype _itemquality _itemgrade _validminigame _itemassetdata) (break `ItemDataStruct` _returnvalue))
        (return _id _itemtype _itemquality _itemgrade _validminigame _itemassetdata)))))

(fn `InteractionTrace`
  (bind _returnvalue (`GameplayStatics.GetPlayerCameraManager` 0))
  (bind _returnvalue_2 (`Actor.K2_GetActorLocation` _returnvalue))
  ;[1 0.7549 0 0.5] Temp until we get MyInteractionComp, Should be easy merge/Replasement from whats here
  (bind (_outhit _returnvalue_3) (`KismetSystemLibrary.SphereTraceSingle` _returnvalue_2 (+ _returnvalue_2 (* (`Actor.GetActorForwardVector` _returnvalue) (`self.InteractionRange`))) 15.0 "TraceTypeQuery3" false (`|MakeArray` (`self.GetOwner`))))
  ;; If Actor not a new one ignore and if no actor is looked at set look actor to non
  (if _returnvalue_3
    (bind (_bblockinghit _binitialoverlap _time _distance _location _impactpoint _normal _impactnormal _physmat _hitactor) (`GameplayStatics.BreakHitResult` _outhit))
    (if (!= _hitactor (`self.LookAtActor`))
      (bind _output_get (set `self.LookAtActor` _hitactor))
      ; Print data found on valid actor
      (bind _message (message `/Game/Code/Core/Inventory/IInteractInterface.LookAt` _output_get))
      (`KismetSystemLibrary.PrintString` (`KismetTextLibrary.Conv_TextToString` _message)))
    (else
      (set `self.LookAtActor` null))))

(fn `RemoveFromInventory`
  (params (Index :type Integer) (RemoveCompletely :type Boolean))
  (locals (LocalItem :type Name) (LocalQuantity :type Integer))
  (bind (_output_itemid _output_quantity) (break `/Game/Code/Core/Inventory/FSlotStruct` (`|GetArrayItem` (`self.Content`) Index)))
  ; Gets a copy of local Inventory slots item ID and quantity
  (set `local.LocalItem` _output_itemid)
  (set `local.LocalQuantity` _output_quantity)
  (`|ExecutionSequence`
    (:`then_0`
      ; Remove Item from slot
      (`KismetArrayLibrary.Array_Set` (`self.Content`) (`local.Index`) (make `/Game/Code/Core/Inventory/FSlotStruct` "None"))
      (if (not (`local.RemoveCompletely`))
        (`self.ServerDropItem` (`local.LocalItem`) (`local.LocalQuantity`))))
    (:`then_1`
      (`self.MC_Update`))))

(fn `TransferSlots`
  (params (SourceIndex :type Integer) (SourceInventory :type "/Game/Code/Core/Inventory/BP_InventorySystem Object Reference") (DestinationIndex :type Integer))
  (locals (LocalSlotContent :type "/Game/Code/Core/Inventory/FSlotStruct Structure"))
  ; Gets a copy and stores source inventory
  (set `local.LocalSlotContent` (`|GetArrayItem` (`/Game/Code/Core/Inventory/BP_InventorySystem.Content` SourceInventory) SourceIndex))
  (if (< DestinationIndex 0)
    _
    (elif (not (== (`.ItemID_2_9A35EB514A7E0F49F31B1696D16693F0` (break `/Game/Code/Core/Inventory/FSlotStruct` (`local.LocalSlotContent`))) (`.ItemID_2_9A35EB514A7E0F49F31B1696D16693F0` (break `/Game/Code/Core/Inventory/FSlotStruct` (`|GetArrayItem` (`self.Content`) (`local.DestinationIndex`))))))
      ; Change Inventory
      ;; Swap items of source and target inventory
      (`KismetArrayLibrary.Array_Set` (`/Game/Code/Core/Inventory/BP_InventorySystem.Content` (`local.SourceInventory`)) (`local.SourceIndex`) (`|GetArrayItem` (`self.Content`) (`local.DestinationIndex`)))
      (`KismetArrayLibrary.Array_Set` (`self.Content`) (`local.DestinationIndex`) (`local.LocalSlotContent`))
      ;; Update source and target inventory
      (`self.MC_Update`)
      (`self.MC_Update` (`local.SourceInventory`)))))