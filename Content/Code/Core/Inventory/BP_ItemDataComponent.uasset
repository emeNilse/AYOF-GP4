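; Actor component that makes its owner an item pickup, feeding an item ID and quantity into the interacting player's inventory.
; On interaction it calls AddToInventory on the player's InventorySystem, then sends the owner a respawn message on success rather than destroying it.
; On failure it can start an inventory-full dialogue and prints a test message.
; BeginPlay turns off replication on the owner, and LookAt returns an empty message.
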(event `self.ReceiveBeginPlay`
  (`Actor.SetReplicates` (`self.GetOwner`) false))

(event `/Game/Code/Core/Inventory/IInteractInterface.InteractWith`
  (params (PlayerCharacter :type "/Game/Code/Player/BP_Character Object Reference"))
  (bind _inventorysystem (`/Game/Code/Player/BP_Character.InventorySystem` PlayerCharacter))
  (bind (_itemid_datatable _itemid_rowname) (break `DataTableRowHandle` (`self.ItemID`)))
  ; If item is valid Add assosiated Item ID to inventory
  (`/Engine/EditorBlueprintResources/StandardMacros.IsValid` _inventorysystem
    (:`Is Valid`
      (bind _success (`/Game/Code/Core/Inventory/BP_InventorySystem.AddToInventory` _inventorysystem _itemid_rowname (`self.Quantity`)))
      (if _success
        ;[1 0.7351 0 0.5] TODO:: find better way than destroy actor
        (message `/Game/Code/Interactables/ItemIngridients/BPI_ItemSpawner.Respawn` (`self.GetOwner`))
        (else
          (if (`self.Show dialogue on inventory full`)
            (`DialogueEventComponent.StartDialogueEvent` (`self.BP_DialogueComponent`) (`self.InventoryFull Dialogue`) false))
          ;[1 0.773 0 0.5] Testing
          (`KismetSystemLibrary.PrintText` "Intereacted With Object. Add to inventory returned fail"))))))

(fn `LookAt`
  (returns (Message :type Text) (SM :type "StaticMeshComponent Object Reference"))
  (return "" null))