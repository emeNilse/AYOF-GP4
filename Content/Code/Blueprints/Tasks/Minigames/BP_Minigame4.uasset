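; Two-player task minigame where spinning the thumbstick is meant to charge motor energy to 100, shown on per-player progress bars.
; Tick, after a short delay, zeroes MotorEnergy and WinValue, then updates the active player's bar; reaching 100 leads only to a DoOnce.
; Stick-angle spin detection, widget show/hide with Enhanced Input context swaps, and state reset are all unwired, so they never run.
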(event `self.ReceiveTick`
  (params (DeltaSeconds :type "Float (single-precision)"))
  ;[0 0.512 1 0.5] Logic
  ;; reads the value from game containern and set a new value from the minigame
  (`KismetSystemLibrary.Delay` 0.2)
  (bind _output_get (set `self.MotorEnergy` 0.0))
  (set `self.WinValue` _output_get)
  (if (`self.Active`)
    ;; Checks the player ID
    (switch `int` (`self.PlayerID`)
      (:`0`
        ;; Set percent for Player 1
        (`ProgressBar.SetPercent` (`/Game/Code/Blueprints/Tasks/Minigames/W_Minigame4P1.ProgressBar1` (`self.W Minigame 4 P1`)) (/ (`self.WinValue`) 100.0)))
      (:`1`
        ;; Set percent for Player 2
        (`ProgressBar.SetPercent` (`/Game/Code/Blueprints/Tasks/Minigames/W_Minigame4P2.ProgressBar2` (`self.W Minigame 4 P2`)) (/ (`self.WinValue`) 100.0))))
    ;; Finished the task
    (if (== (`self.WinValue`) 100.0)
      (`/Engine/EditorBlueprintResources/StandardMacros.DoOnce` false))))

(event `ResetSound`
  ;[0 0.512 1 0.5] Logic
  ;; Finished the task
  (`/Engine/EditorBlueprintResources/StandardMacros.DoOnce` false :!via `Reset`
    (:`Completed`
      (`GameplayStatics.PlaySound2D` null 1.0 1.0 0.0 null null))))

(fn `CheckPlayerID`
  (params (`Sending Player` :type "Object Object Reference")))

(fn `UserConstructionScript`)