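; Timing minigame task for two local players, each with their own widget containing a radial slider and progress bar.
; While active, Tick loops the slider and raises progress for the player ID, triggering a DoOnce when both max out.
; Unconnected chains hold the widget and Enhanced Input context swapping, plus press scoring that rewards mid-range slider timing and penalizes misses.
; ResetSound resets that DoOnce, whose completion plays a sound.
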(event `ResetSound`
  ;[0 0.512 1 0.5] Logic
  ;; Play sounds if the progressbar reaches 100
  (goto _label :!via `Reset`))

(event `self.ReceiveTick`
  (params (DeltaSeconds :type "Float (single-precision)"))
  (bind _w_minigame_5_p2 (`self.W Minigame 5 P2`))
  (bind _w_minigame_5_p1 (`self.W Minigame 5 P1`))
  ;[0 0.512 1 0.5] Logic
  ;; Adds to the slider value and progress bar
  (if (`self.Active`)
    (`KismetSystemLibrary.Delay` 0.05)
    (switch `int` (`self.PlayerID`)
      (:`0`
        (set `self.Progressbar` 0.0)
        ;;; Player 1
        (set `self.SliderValue` (`KismetMathLibrary.FClamp` (+ (`self.SliderValue`) 3.0) 0.0 100.0))
        ;;;;[0.8802 0.7385 0.04082 0.5] How fast slidern go
        (set `self.Progressbar` (+ (`self.Progressbar`) 2.0))
        (`ProgressBar.SetPercent` (`/Game/Code/Blueprints/Tasks/Minigames/W_Minigame5P1.ProgressBar` _w_minigame_5_p1) (/ (`self.Progressbar`) 100.0))
        (`RadialSlider.SetValue` (`/Game/Code/Blueprints/Tasks/Minigames/W_Minigame5P1.RadialSlider_0` _w_minigame_5_p1) (/ (`self.SliderValue`) 100.0))
        (if (<= 100.0 (`self.SliderValue`))
          (set `self.SliderValue` 0.0)
          (if (<= 100.0 (`self.Progressbar`))
            ;; Play sounds if the progressbar reaches 100
            (`/Engine/EditorBlueprintResources/StandardMacros.DoOnce` false :!label _label
              (:`Completed`
                (`GameplayStatics.PlaySound2D` null 1.0 1.0 0.0 null null))))))
      (:`1`
        (set `self.Progressbar` 0.0)
        ;;; Player 2
        (set `self.SliderValue` (`KismetMathLibrary.FClamp` (+ (`self.SliderValue`) 3.0) 0.0 100.0))
        ;;;;[0.8802 0.7385 0.04082 0.5] How fast slidern go
        (set `self.Progressbar` (+ (`self.Progressbar`) 2.0))
        (`ProgressBar.SetPercent` (`/Game/Code/Blueprints/Tasks/Minigames/W_Minigame5P2.ProgressBar2` _w_minigame_5_p2) (/ (`self.Progressbar`) 100.0))
        (`RadialSlider.SetValue` (`/Game/Code/Blueprints/Tasks/Minigames/W_Minigame5P2.RadialSlider_0` _w_minigame_5_p2) (/ (`self.SliderValue`) 100.0))
        (if (<= 100.0 (`self.SliderValue`))
          (set `self.SliderValue` 0.0)
          (if (<= 100.0 (`self.Progressbar`))
            (goto _label)))))))

(fn `CheckPlayerID`
  (params (`Sending Player` :type "Object Object Reference")))

(fn `UserConstructionScript`)