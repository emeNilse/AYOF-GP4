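; Minigame 3 task actor: a balance game for either of two players, where keeping a drifting slider near the centre fills a progress bar.
; Tick updates that player's widget and runs DoOnce-gated, delayed steps that raise or lower progress and randomly nudge the slider.
; A full bar resets values, plays a sound and re-arms the gate.
; Widget show/hide, input-context swapping and slider button logic exist but are unwired.
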(event `self.ReceiveTick`
  (params (DeltaSeconds :type "Float (single-precision)"))
  (bind _slider1 (`self.Slider1`))
  (bind _slider2 (`self.Slider2`))
  ;[0 0.512 1 0.5] Logic
  ;; Adds or removes value to the progressbar when the slider is or is not in between the fill area
  (if (`self.Active`)
    (switch `int` (`self.PlayerID`)
      (:`0`
        ;;; Sets Slider value for Player 1
        (`Slider.SetValue` (`/Game/Code/Blueprints/Tasks/Minigames/W_Minigame3P1.Slider1` (`self.W_Minigame3P1`)) (/ (`self.Slider1`) 100.0))
        ;;; Player 1
        (`/Engine/EditorBlueprintResources/StandardMacros.DoOnce` false :!label _label
          (:`Completed`
            (if (== (<= _slider1 57.0) (>= _slider1 43.0))
              (set `self.ProgressBar1` (`KismetMathLibrary.FClamp` (+ (`self.ProgressBar1`) 8.0) 0.0 100.0))
              (else
                (set `self.ProgressBar1` (`KismetMathLibrary.FClamp` (- (`self.ProgressBar1`) 4.0) 0.0 100.0))))
            (if (== (`self.ProgressBar1`) 100.0)
              _
              (else
                (`KismetSystemLibrary.Delay` 0.3)
                ;; Randomly adds or removes value from the slider
                ;;; Player 1
                (if (`KismetMathLibrary.RandomBool`)
                  (set `self.Slider1` (- (`self.Slider1`) 2.0))
                  (else
                    (set `self.Slider1` (+ (`self.Slider1`) 2.0))))
                ;; Sets the percent on the progressbar
                (switch `int` (`self.PlayerID`) :!label _label_2
                  (:`0`
                    (`ProgressBar.SetPercent` (`/Game/Code/Blueprints/Tasks/Minigames/W_Minigame3P1.ProgressBar1` (`self.W_Minigame3P1`)) (/ (`self.ProgressBar1`) 100.0)))
                  (:`1`
                    (`ProgressBar.SetPercent` (`/Game/Code/Blueprints/Tasks/Minigames/W_Minigame3P2.ProgressBar2` (`self.W Minigame 3P2`)) (/ (`self.ProgressBar2`) 100.0))))
                (switch `int` (`self.PlayerID`) :!label _label_3
                  (:`0`
                    (goto _label :!via `Reset`))
                  (:`1`
                    (goto _label_4 :!via `Reset`))))))))
      (:`1`
        ;;; Sets Slider value for Player 2
        (`Slider.SetValue` (`/Game/Code/Blueprints/Tasks/Minigames/W_Minigame3P2.Slider2` (`self.W Minigame 3P2`)) (/ (`self.Slider2`) 100.0))
        ;;; Player 2
        (`/Engine/EditorBlueprintResources/StandardMacros.DoOnce` false :!label _label_4
          (:`Completed`
            (if (== (<= _slider2 57.0) (>= _slider2 43.0))
              (set `self.ProgressBar2` (`KismetMathLibrary.FClamp` (+ (`self.ProgressBar2`) 8.0) 0.0 100.0))
              (else
                (set `self.ProgressBar2` (`KismetMathLibrary.FClamp` (- (`self.ProgressBar2`) 4.0) 0.0 100.0))))
            (if (== (`self.ProgressBar2`) 100.0)
              _
              (else
                (`KismetSystemLibrary.Delay` 0.3)
                ;;; Player 2
                (if (`KismetMathLibrary.RandomBool`)
                  (set `self.Slider2` (- (`self.Slider2`) 2.0))
                  (goto _label_2)
                  (else
                    (set `self.Slider2` (+ (`self.Slider2`) 2.0))
                    (goto _label_2)))))))))
    ;; Finished the task
    (set `self.Active` false)
    (set `self.ProgressBar1` 0.1)
    (set `self.ProgressBar2` 0.1)
    (set `self.Slider1` 50.0)
    (set `self.Slider2` 50.0)
    (`GameplayStatics.PlaySound2D` null 1.0 1.0 0.0 null null)
    (`KismetSystemLibrary.PrintString` "Done 2")
    (`self.IWANTTOCRY`)))

(event `IWANTTOCRY`
  ;[0 0.512 1 0.5] Logic
  (goto _label_3))

(fn `CheckPlayerID`
  (params (SendingPlayer :type "Object Object Reference")))

(fn `UserConstructionScript`)