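; Blueprint for a two-player button-mashing task minigame in which each player fills a progress bar that drains over time.
; While active, Tick uses a DoOnce and Delay loop to drain both values and update the current player's widget.
; Button-press, widget and input mapping-context swap chains branch on player ID, but none has a triggering event.
; Only player 2's branch handles completion; CheckPlayerID is empty.
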(event `self.ReceiveTick`
  (params (DeltaSeconds :type "Float (single-precision)"))
  ;[0 0.512 1 0.5] Logic
  ;; Decreases the progressbar value
  (if (`self.Active`)
    (`/Engine/EditorBlueprintResources/StandardMacros.DoOnce` false :!label _label
      (:`Completed`
        (set `self.Progressbar1` (`KismetMathLibrary.FClamp` (- (`self.Progressbar1`) 2.0) 0.0 100.0))
        (set `self.Progressbar2` (`KismetMathLibrary.FClamp` (- (`self.Progressbar2`) 2.0) 0.0 100.0))
        ;; Set the percent for the progressbars
        (`KismetSystemLibrary.Delay` 0.1)
        (switch `int` (`self.PlayerID`)
          (:`0`
            (`ProgressBar.SetPercent` (`/Game/Code/Blueprints/Tasks/Minigames/W_Minigame1.ProgressBar1` (`self.MiniGameWidgetP1`)) (/ (`self.Progressbar1`) 100.0))
            (goto _label :!via `Reset`))
          (:`1`
            (`ProgressBar.SetPercent` (`/Game/Code/Blueprints/Tasks/Minigames/W_Minigame1P2.ProgressBar2` (`self.MiniGameWidgetP2`)) (/ (`self.Progressbar2`) 100.0))
            (goto _label :!via `Reset`)))))))

(fn `CheckPlayerID`
  (params (SendingPlayer :type "Object Object Reference")))

(fn `UserConstructionScript`)