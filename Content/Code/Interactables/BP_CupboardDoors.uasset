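; BP_CupboardDoors is an interactable pair of cupboard doors that swing open or closed when a player interacts, and supplies its name as look-at text.
; OnInteract calls Open&Close, where a FlipFlop plays or reverses a timeline that lerps both doors' yaw in opposite directions.
; Each use spawns an attached MetaSound, triggering "Open" as opening starts and "Close" once the reverse finishes.
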(event `Open&Close`
  (bind _returnvalue (`GameplayStatics.SpawnSoundAttached` "/Game/Audio/MetaSounds/SFX/MS_GenericOpenClose.MS_GenericOpenClose" (`self.Right`) "None" (0.0 0.0 0.0) (struct) "KeepRelativeOffset" false 1.0 1.0 0.0 null null))
  (set `self.AudioComponent` _returnvalue)
  (bind _isa (`/Engine/EditorBlueprintResources/StandardMacros.FlipFlop`)
    (:`A`
      (set `self.Is A` _isa)
      (`AudioParameterControllerInterface.SetTriggerParameter` (`self.AudioComponent`) "Open")
      (bind (_direction _newtrack_0) (`Timeline|Cupboard Doors` :!label _label)
        (:`Update`
          (`SceneComponent.K2_SetRelativeRotation` (`self.Left`) (`KismetMathLibrary.MakeRotator` 0.0 0.0 (`KismetMathLibrary.Lerp` 10.0 90.0 _newtrack_0)) false false)
          (`SceneComponent.K2_SetRelativeRotation` (`self.Right`) (`KismetMathLibrary.MakeRotator` 0.0 0.0 (`KismetMathLibrary.Lerp` 0.0 -90.0 _newtrack_0)) false false))
        (:`Finished`
          (if (not (`self.Is A`))
            (`AudioParameterControllerInterface.SetTriggerParameter` (`self.AudioComponent`) "Close")))))
    (:`B`
      (set `self.Is A` _isa)
      (goto _label :!via `Reverse`))))

(fn `LookAt`
  (returns (Message :type Text) (SM :type "StaticMeshComponent Object Reference"))
  (return (`KismetTextLibrary.Conv_NameToText` (`self.Name`)) null))

(fn `OnInteract`
  (params (interactingPlayer :type "MyPlayerController Object Reference"))
  (`self.Open&Close`)
  (`parent.OnInteract` interactingPlayer))

(fn `UserConstructionScript`)