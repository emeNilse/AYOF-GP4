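; BP_Knife is an interactable knife that plays a chopping animation and sound, driven by externally callable functions.
; ReadyAnimation moves it to a hard-coded cutting pose and primes the cut animation, TriggerAnimation plays the cut with sound, and StopAnimation halts it and sets a separate resting pose.
; BeginPlay caches StartPosition, but StopAnimation uses hard-coded values instead, as do the other pose and sound placements.
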(event `self.ReceiveBeginPlay`
  (bind _returnvalue_location (`KismetMathLibrary.BreakTransform` (`self.GetTransform`)))
  (bind (_returnvalue_location_2 _returnvalue_rotation) (`KismetMathLibrary.BreakTransform` (`SceneComponent.K2_GetComponentToWorld` (`self.SkeletalMesh`))))
  (set `self.StartPosition` (`KismetMathLibrary.MakeTransform` _returnvalue_location _returnvalue_rotation)))

(fn `ReadyAnimation`
  (bind _skeletalmesh (`self.SkeletalMesh`))
  (`SceneComponent.K2_SetRelativeTransform` (`self.DefaultSceneRoot`) (`KismetMathLibrary.MakeTransform` (-835.0 -50.0 130.0) (struct :`Yaw` 180.0)) false false)
  (`SkeletalMeshComponent.PlayAnimation` _skeletalmesh "/Game/Art/1-Assets/Decorations/Animated/Knife_Anim/SKM_Knife_Interactable_Anim_SK_KnifeCut.SKM_Knife_Interactable_Anim_SK_KnifeCut" false)
  (`SkeletalMeshComponent.Stop` _skeletalmesh))

(fn `StopAnimation`
  (`SkeletalMeshComponent.Stop` (`self.SkeletalMesh`))
  (`SceneComponent.K2_SetRelativeTransform` (`self.DefaultSceneRoot`) (`KismetMathLibrary.MakeTransform` (-825.0 -60.0 130.0) (struct :`Pitch` 90.0 :`Yaw` 90.0 :`Roll` -90.0)) false false))

(fn `TriggerAnimation`
  (`SkeletalMeshComponent.PlayAnimation` (`self.SkeletalMesh`) "/Game/Art/1-Assets/Decorations/Animated/Knife_Anim/SKM_Knife_Interactable_Anim_SK_KnifeCut.SKM_Knife_Interactable_Anim_SK_KnifeCut" false)
  (`GameplayStatics.SpawnSoundAtLocation` "/Game/Audio/MetaSounds/SFX/MS_Chopping.MS_Chopping" (-835.0 -50.0 130.0) (struct) 5.0 5.0 0.0 null null))

(fn `UserConstructionScript`)