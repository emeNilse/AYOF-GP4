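; Possessable cooking station where the player mixes Batter and CakeCream through staged clicks and minigames.
; Interacting opens its inventory container; clicking ingredient meshes raises counts shown on text renders.
; Jump advances stages: correct counts start the first minigame, then mixing minigames award each product to the player's inventory.
; Player-inventory ingredient checking is disconnected, as is RemoveItem's actual removal; possession instead removes items from the station's own inventory.
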(event `Event InteractWith`
  (bind _asbp_player_controller (cast `/Game/Code/Core/BP_PlayerController` (`GameplayStatics.GetPlayerController` 0)))
  (`/Game/Code/UI/UI_Inventory/W_PlayerHUD.ShowContainer` (`/Game/Code/Core/BP_PlayerController.HUD` _asbp_player_controller) (`self.BP_InventorySystem`)))

(event `self.ReceiveBeginPlay`
  (bind _ingredients (`self.Ingredients`))
  (bind _cream (`self.Cream`))
  ; Hide ingredients at start
  (`SceneComponent.SetVisibility` _ingredients false true)
  (set `self.Stage` 1)
  (`SceneComponent.SetVisibility` _ingredients true false)
  (`self.HideText`)
  (`PrimitiveComponent.SetCollisionEnabled` _cream "NoCollision")
  (`PrimitiveComponent.SetCollisionResponseToAllChannels` _cream "ECR_Ignore"))

(event `self.ReceiveUnpossessed`
  (params (OldController :type "Controller Object Reference"))
  (`self.HideText`))

(event `self.ReceivePossessed`
  (params (NewController :type "Controller Object Reference"))
  (set `self.New Controller` NewController)
  (`|ExecutionSequence`
    (:`then_0`
      (`self.ResetAllAMounts`)
      (if (== (`self.Stage`) 1)
        (`self.CheckIngredientsBaseFunction`)))
    (:`then_1`
      (if (== (`self.Stage`) 1)
        (`self.ShowText`)
        (elif (== (`self.Stage`) 3)
          (`self.HandleCreamText`)
          (`self.CheckCream`))))))

(event `self.Sugar.OnClicked`
  (params (TouchedComponent :type "PrimitiveComponent Object Reference") (ButtonPressed :type "Key Structure"))
  ; Handle Click
  (if (`self.LockClicks`)
    _
    (elif (`SceneComponent.IsVisible` (`self.Sugar`))
      (bind _result (`/Engine/EditorBlueprintResources/StandardMacros.IncrementInt` (`self.SugarAmount`))
        (:`  `
          (set `self.SugarAmount` _result)
          (`self.ShowText` :!label _label))))))

(event `self.Flour.OnClicked`
  (params (TouchedComponent :type "PrimitiveComponent Object Reference") (ButtonPressed :type "Key Structure"))
  ; Handle Click
  (if (`self.LockClicks`)
    _
    (elif (`SceneComponent.IsVisible` (`self.Flour`))
      (bind _result (`/Engine/EditorBlueprintResources/StandardMacros.IncrementInt` (`self.FlourAmount`))
        (:`  `
          (set `self.FlourAmount` _result)
          (goto _label))))))

(event `self.Powder.OnClicked`
  (params (TouchedComponent :type "PrimitiveComponent Object Reference") (ButtonPressed :type "Key Structure"))
  ; Handle Click
  (if (`self.LockClicks`)
    _
    (elif (`SceneComponent.IsVisible` (`self.Powder`))
      (bind _result (`/Engine/EditorBlueprintResources/StandardMacros.IncrementInt` (`self.PowderAmount`))
        (:`  `
          (set `self.PowderAmount` _result)
          (goto _label))))))

(event `self.Eggs.OnClicked`
  (params (TouchedComponent :type "PrimitiveComponent Object Reference") (ButtonPressed :type "Key Structure"))
  ; Handle Click
  (if (`self.LockClicks`)
    _
    (elif (`SceneComponent.IsVisible` (`self.Eggs`))
      (bind _result (`/Engine/EditorBlueprintResources/StandardMacros.IncrementInt` (`self.EggsAmount`))
        (:`  `
          (set `self.EggsAmount` _result)
          (goto _label))))))

(event `self.Cream.OnClicked`
  (params (TouchedComponent :type "PrimitiveComponent Object Reference") (ButtonPressed :type "Key Structure"))
  ; Handle Click
  (if (`self.LockClicks`)
    _
    (elif (`SceneComponent.IsVisible` (`self.Cream`))
      (bind _result (`/Engine/EditorBlueprintResources/StandardMacros.IncrementInt` (`self.CreamAmount`))
        (:`  `
          (set `self.CreamAmount` _result)
          (`self.HandleCreamText`))))))

(event `EnhancedInput|/Game/Code/Input/Actions/IA_Jump`
  (params (ActionValue :type Boolean) (ElapsedSeconds :type "Float (double-precision)") (TriggeredSeconds :type "Float (double-precision)") (InputAction :type "InputAction Object Reference" :default "/Game/Code/Input/Actions/IA_Jump.IA_Jump"))
  (:`Completed`
    (if (== (`self.Stage`) 1)
      (bind _correct (`self.CheckSequence`))
      (if _correct
        (set `self.LockClicks` true)
        (bind _returnvalue (`|SpawnActorFromClass` (`self.Minigame_1`) (`KismetMathLibrary.MakeTransform` (`SceneComponent.K2_GetComponentLocation` (`self.Camera`))) "Undefined" "MultiplyWithRoot" null null))
        (bind _asbp_mg_cutting (cast `/Game/Code/MiniGames/BP_MG_Cutting` _returnvalue)
          (:`then`
            (add `/Game/Code/MiniGames/BP_MG_Cutting.OnMinigameCompleted` _asbp_mg_cutting (delegate `OnFirstCompleted`)))
          (:`CastFailed`
            (`SceneComponent.SetVisibility` (`self.Eggs`) false false :!label _label_2)
            (set `self.Stage` 2))))
      (elif (== (`self.Stage`) 2)
        (`SceneComponent.SetVisibility` (`self.Sugar`) false false)
        (`SceneComponent.SetVisibility` (`self.Powder`) false false)
        (`SceneComponent.SetVisibility` (`self.Flour`) false false)
        (`self.HideText`)
        (bind _returnvalue_2 (`|SpawnActorFromClass` (`self.Minigame_2`) (`KismetMathLibrary.MakeTransform` (`SceneComponent.K2_GetComponentLocation` (`self.Camera`))) "Undefined" "MultiplyWithRoot" null null))
        (bind _asbp_mg_mixing (cast `/Game/Code/MiniGames/BP_MG_Mixing` _returnvalue_2)
          (:`then`
            (add `/Game/Code/MiniGames/BP_MG_Mixing.OnMinigameCompleted` _asbp_mg_mixing (delegate `OnSecondFinished`)))
          (:`CastFailed`
            (set `self.Stage` 3 :!label _label_3)
            (set `self.LockClicks` false)
            (`self.HandleCreamText`)
            (`self.CheckCream`)
            (`self.AddItem` "Batter")))
        (elif (== (`self.Stage`) 3)
          (if (== (`self.CreamAmount`) 2)
            (bind _returnvalue_3 (`|SpawnActorFromClass` (`self.Minigame_2`) (`KismetMathLibrary.MakeTransform` (`SceneComponent.K2_GetComponentLocation` (`self.Camera`))) "Undefined" "MultiplyWithRoot" null null))
            (bind _asbp_mg_mixing_2 (cast `/Game/Code/MiniGames/BP_MG_Mixing` _returnvalue_3)
              (:`then`
                (add `/Game/Code/MiniGames/BP_MG_Mixing.OnMinigameCompleted` _asbp_mg_mixing_2 (delegate `OnThirdFinished`)))
              (:`CastFailed`
                (`self.AddItem` "CakeCream" :!label _label_4)
                (set `self.Stage` 4)
                (`SceneComponent.SetVisibility` (`self.Ingredients`) false true)
                (`self.HideText`)))))))))

(event `OnFirstCompleted`
  (params (Quality :type "Float (double-precision)"))
  (goto _label_2))

(event `OnSecondFinished`
  (params (Quality :type "Float (double-precision)"))
  (goto _label_3))

(event `OnThirdFinished`
  (params (Quality :type "Float (double-precision)"))
  (goto _label_4))

(fn `AddItem`
  (params (ItemID :type Name))
  (bind _asmy_player_controller (cast `MyPlayerController` (`GameplayStatics.GetPlayerController` 0)))
  (`/Game/Code/Core/Inventory/BP_InventorySystem.AddToInventory` (`self.GetComponentByClass` (`MyPlayerController.CharacterPawn` _asmy_player_controller) "/Game/Code/Core/Inventory/BP_InventorySystem.BP_InventorySystem_C") ItemID 1))

(fn `CheckCream`
  (locals (DeleteCream :type Boolean))
  (bind _cream (`self.Cream`))
  (bind _asmy_player_controller (cast `MyPlayerController` (`GameplayStatics.GetPlayerController` 0)))
  (for _array_element (`/Game/Code/Core/Inventory/BP_InventorySystem.Content` (`self.GetComponentByClass` (`MyPlayerController.CharacterPawn` _asmy_player_controller) "/Game/Code/Core/Inventory/BP_InventorySystem.BP_InventorySystem_C"))
    (if (== (`.ItemID_2_9A35EB514A7E0F49F31B1696D16693F0` (break `/Game/Code/Core/Inventory/FSlotStruct` _array_element)) (`|GetArrayItem` (`self.Contents`) 4))
      (if (not (`SceneComponent.IsVisible` (`self.Cream`)))
        (`SceneComponent.SetVisibility` (`self.Cream`) true false)
        (set `self.CreamAmount` 0)
        (`PrimitiveComponent.SetCollisionEnabled` _cream "QueryAndPhysics")
        (`PrimitiveComponent.SetCollisionResponseToAllChannels` _cream "ECR_Block")
        (set `local.DeleteCream` true))))
  (if (`local.DeleteCream`)
    (`self.RemoveItem` "RawCream")))

(fn `CheckIngredients`
  (locals (ID :type Name) (DeleteEgg :type Boolean) (DeleteFlour :type Boolean) (DeletePowder :type Boolean) (DeleteSugar :type Boolean))
  (bind _asmy_player_controller (cast `MyPlayerController` (`GameplayStatics.GetPlayerController` 0)))
  (for _array_element (`/Game/Code/Core/Inventory/BP_InventorySystem.Content` (`self.GetComponentByClass` (`MyPlayerController.CharacterPawn` _asmy_player_controller) "/Game/Code/Core/Inventory/BP_InventorySystem.BP_InventorySystem_C"))
    (bind _itemid (break `/Game/Code/Core/Inventory/FSlotStruct` _array_element))
    (set `local.ID` _itemid)
    (if (== _itemid (`|GetArrayItem` (`self.Contents`)))
      (if (not (`SceneComponent.IsVisible` (`self.Eggs`)))
        (`SceneComponent.SetVisibility` (`self.Eggs`) true false)
        (set `local.DeleteEgg` true))
      (elif (== (`local.ID`) (`|GetArrayItem` (`self.Contents`) 1))
        (if (not (`SceneComponent.IsVisible` (`self.Sugar`)))
          (`SceneComponent.SetVisibility` (`self.Sugar`) true false)
          (set `local.DeleteSugar` true))
        (elif (== (`local.ID`) (`|GetArrayItem` (`self.Contents`) 2))
          (if (not (`SceneComponent.IsVisible` (`self.Powder`)))
            (`SceneComponent.SetVisibility` (`self.Powder`) true false)
            (set `local.DeletePowder` true))
          (elif (== (`local.ID`) (`|GetArrayItem` (`self.Contents`) 3))
            (if (not (`SceneComponent.IsVisible` (`self.Flour`)))
              (`SceneComponent.SetVisibility` (`self.Flour`) true false)
              (set `local.DeleteFlour` true)))))))
  (if (`local.DeleteEgg`)
    (`self.RemoveItem` "Egg"))
  (if (`local.DeleteFlour`)
    (`self.RemoveItem` "Flour"))
  (if (`local.DeleteSugar`)
    (`self.RemoveItem` "Sugar"))
  (if (`local.DeletePowder`)
    (`self.RemoveItem` "Powder")))

(fn `CheckIngredientsBaseFunction`
  (locals (ItemID :type Name) (DeleteItemOne :type Boolean) (DeleteItemTwo :type Boolean) (DeleteItemThree :type Boolean) (DeleteItemFour :type Boolean) (DeleteItemFive :type Boolean))
  (for _array_element (`/Game/Code/Core/Inventory/BP_InventorySystem.Content` (`self.BP_InventorySystem`))
    (set `local.ItemID` (`.ItemID_2_9A35EB514A7E0F49F31B1696D16693F0` (break `/Game/Code/Core/Inventory/FSlotStruct` _array_element)))
    (if (== (`local.ItemID`) (`|GetArrayItem` (`self.Contents`)))
      (set `local.DeleteItemOne` true)
      (elif (== (`local.ItemID`) (`|GetArrayItem` (`self.Contents`) 1))
        (set `local.DeleteItemTwo` true)
        (elif (== (`local.ItemID`) (`|GetArrayItem` (`self.Contents`) 2))
          (set `local.DeleteItemThree` true)
          (elif (== (`local.ItemID`) (`|GetArrayItem` (`self.Contents`) 3))
            (set `local.DeleteItemFour` true)
            (elif (== (`local.ItemID`) (`|GetArrayItem` (`self.Contents`) 4))
              (set `local.DeleteItemFive` true)))))))
  (if (`local.DeleteItemOne`)
    (`/Game/Code/Core/Inventory/BP_InventorySystem.ServerRemove` (`self.BP_InventorySystem`) 0 true)
    (elif (`local.DeleteItemTwo`)
      (`/Game/Code/Core/Inventory/BP_InventorySystem.ServerRemove` (`self.BP_InventorySystem`) 1 true)
      (elif (`local.DeleteItemThree`)
        (`/Game/Code/Core/Inventory/BP_InventorySystem.ServerRemove` (`self.BP_InventorySystem`) 2 true)
        (elif (`local.DeleteItemFour`)
          (`/Game/Code/Core/Inventory/BP_InventorySystem.ServerRemove` (`self.BP_InventorySystem`) 3 true)
          (elif (`local.DeleteItemFive`)
            (`/Game/Code/Core/Inventory/BP_InventorySystem.ServerRemove` (`self.BP_InventorySystem`) 4 true)))))))

(fn `CheckSequence`
  (returns (Correct :type Boolean))
  (if (== (`self.SugarAmount`) 2)
    (if (== (`self.PowderAmount`) 2)
      (if (== (`self.FlourAmount`) 2)
        (if (== (`self.EggsAmount`) 2)
          (return true)
          (else
            (return false)))))))

(fn `HandleCreamText`
  (`TextRenderComponent.K2_SetText` (`self.TextRender3`) (`|FormatText` (`|GetArrayItem` (`self.Text`) 6) (`self.CreamAmount`)))
  (`TextRenderComponent.K2_SetText` (`self.TextRender4`) (`|GetArrayItem` (`self.Text`) 5)))

(fn `HideText`
  (bind _output (`|GetArrayItem` (`self.Text`)))
  (`TextRenderComponent.K2_SetText` (`self.TextRender`) _output)
  (`TextRenderComponent.K2_SetText` (`self.TextRender1`) _output)
  (`TextRenderComponent.K2_SetText` (`self.TextRender2`) _output)
  (`TextRenderComponent.K2_SetText` (`self.TextRender3`) _output)
  (`TextRenderComponent.K2_SetText` (`self.TextRender4`) _output))

(fn `RemoveItem`
  (params (ItemID :type Name))
  (bind _asmy_player_controller (cast `MyPlayerController` (`self.New Controller`))
    (:`then`
      (for (_array_element _array_index) (`/Game/Code/Core/Inventory/BP_InventorySystem.Content` (`self.GetComponentByClass` (`MyPlayerController.CharacterPawn` _asmy_player_controller) "/Game/Code/Core/Inventory/BP_InventorySystem.BP_InventorySystem_C"))
        (bind _itemid (break `/Game/Code/Core/Inventory/FSlotStruct` _array_element))
        (`KismetSystemLibrary.PrintString` (`KismetStringLibrary.Conv_NameToString` _itemid))
        (if (== _itemid ItemID)
          _)))
    (:`CastFailed`
      (`KismetSystemLibrary.PrintString` "Cast Failed!"))))

(fn `ResetAllAMounts`
  (set `self.SugarAmount` 0)
  (set `self.PowderAmount` 0)
  (set `self.FlourAmount` 0)
  (set `self.EggsAmount` 0)
  (set `self.CreamAmount` 0))

(fn `ShowText`
  (`TextRenderComponent.K2_SetText` (`self.TextRender`) (`|FormatText` (`|GetArrayItem` (`self.Text`) 1) (`self.EggsAmount`)))
  (`TextRenderComponent.K2_SetText` (`self.TextRender1`) (`|FormatText` (`|GetArrayItem` (`self.Text`) 2) (`self.FlourAmount`)))
  (`TextRenderComponent.K2_SetText` (`self.TextRender2`) (`|FormatText` (`|GetArrayItem` (`self.Text`) 3) (`self.SugarAmount`)))
  (`TextRenderComponent.K2_SetText` (`self.TextRender3`) (`|FormatText` (`|GetArrayItem` (`self.Text`) 4) (`self.PowderAmount`)))
  (`TextRenderComponent.K2_SetText` (`self.TextRender4`) (`|GetArrayItem` (`self.Text`) 5)))

(fn `UserConstructionScript`)