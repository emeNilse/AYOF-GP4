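; Water cooking station that produces a water pitcher through a minigame when possessed.
; On possession it tries to start the minigame, leaving immediately if its current pitcher still exists.
; Finishing the minigame spawns a BP_WaterPitcher slightly offset from the station, stores it as the current pitcher and leaves; the quality result is unused.
; Its overrides of the possession, start and finish functions skip the parent implementations.
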(event `self.ReceivePossessed`
  (params (NewController :type "Controller Object Reference"))
  (`self.OnPossessed`))

(fn `OnMinigameFinished`
  (params (Quality :type "Float (double-precision)"))
  (bind (_returnvalue_x _returnvalue_y _returnvalue_z) (`KismetMathLibrary.BreakVector` (`self.K2_GetActorLocation` (`ActorComponent.GetOwner` (`self.StaticMesh`)))))
  (bind _returnvalue (`|SpawnActorFromClass` "/Game/Code/Interactables/ItemIngridients/BP_WaterPitcher.BP_WaterPitcher_C" (`KismetMathLibrary.MakeTransform` (`KismetMathLibrary.MakeVector` (+ _returnvalue_x -10.0) _returnvalue_y (+ _returnvalue_z -15.0))) "Undefined" "MultiplyWithRoot" null 0.0 null))
  (set `self.CurrentPitcher` _returnvalue)
  (`self.LeaveStation`))

(fn `OnPossessed`
  (`self.TryStartMinigame`))

(fn `TryStartMinigame`
  (returns (isMinigameStartSuccess :type Boolean))
  (`/Engine/EditorBlueprintResources/StandardMacros.IsValid` (`self.CurrentPitcher`)
    (:`Is Valid`
      (`self.LeaveStation`))
    (:`Is Not Valid`
      (`self.SpawnMinigame`))))

(fn `UserConstructionScript`
  (`parent.UserConstructionScript`))