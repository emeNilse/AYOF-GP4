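; Assembling cooking station that shows the items placed in it and adds effects to the minigame inherited from its parent.
; Inventory updates refresh three static meshes from the first three inventory slots via ItemData table lookups, clearing any slot without a matching row.
; A successful minigame start activates a smoke puff and attached assembly sound.
; Finishing deactivates the smoke and sends the sound a Stop trigger before calling the parent.
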(event `self.ReceiveBeginPlay`
  (add `/Game/Code/Core/Inventory/BP_InventorySystem.OnInventoryUpdated` (`self.BP_InventorySystem`) (delegate `UpdateDisplay`)))

(event `UpdateDisplay`
  (`self.DisplayItems`))

(fn `DisplayItems`
  (`|ExecutionSequence`
    (:`then_0`
      (bind _returnvalue (`|GetDataTableRow` "/Game/Code/Core/Inventory/ItemData.ItemData" (`.ItemID_2_9A35EB514A7E0F49F31B1696D16693F0` (break `/Game/Code/Core/Inventory/FSlotStruct` (`|GetArrayItem` (`/Game/Code/Core/Inventory/BP_InventorySystem.Content` (`self.BP_InventorySystem`))))))
        (:`then`
          (`StaticMeshComponent.SetStaticMesh` (`self.Item1`) (`.Mesh` (break `ItemAssetData` (`.ItemAssetData` (break `ItemDataStruct` _returnvalue))))))
        (:`RowNotFound`
          (`StaticMeshComponent.SetStaticMesh` (`self.Item1`) null))))
    (:`then_1`
      (bind _returnvalue_2 (`|GetDataTableRow` "/Game/Code/Core/Inventory/ItemData.ItemData" (`.ItemID_2_9A35EB514A7E0F49F31B1696D16693F0` (break `/Game/Code/Core/Inventory/FSlotStruct` (`|GetArrayItem` (`/Game/Code/Core/Inventory/BP_InventorySystem.Content` (`self.BP_InventorySystem`)) 1))))
        (:`then`
          (`StaticMeshComponent.SetStaticMesh` (`self.Item2`) (`.Mesh` (break `ItemAssetData` (`.ItemAssetData` (break `ItemDataStruct` _returnvalue_2))))))
        (:`RowNotFound`
          (`StaticMeshComponent.SetStaticMesh` (`self.Item2`) null))))
    (:`then_2`
      (bind _returnvalue_3 (`|GetDataTableRow` "/Game/Code/Core/Inventory/ItemData.ItemData" (`.ItemID_2_9A35EB514A7E0F49F31B1696D16693F0` (break `/Game/Code/Core/Inventory/FSlotStruct` (`|GetArrayItem` (`/Game/Code/Core/Inventory/BP_InventorySystem.Content` (`self.BP_InventorySystem`)) 2))))
        (:`then`
          (`StaticMeshComponent.SetStaticMesh` (`self.Item3`) (`.Mesh` (break `ItemAssetData` (`.ItemAssetData` (break `ItemDataStruct` _returnvalue_3))))))
        (:`RowNotFound`
          (`StaticMeshComponent.SetStaticMesh` (`self.Item3`) null))))))

(fn `LookAtBackup`
  (returns (Message :type Text))
  (return ""))

(fn `OnMinigameFinished`
  (params (Quality :type "Float (double-precision)"))
  (`ActorComponent.Deactivate` (`self.SmokePuff`))
  (`AudioParameterControllerInterface.SetTriggerParameter` (`self.AudioComponent`) "Stop")
  (`parent.OnMinigameFinished` Quality))

(fn `TryStartMinigame`
  (returns (isMinigameStartSuccess :type Boolean))
  (bind _isminigamestartsuccess (`parent.TryStartMinigame`))
  (if _isminigamestartsuccess
    (`ActorComponent.Activate` (`self.SmokePuff`) true)
    (bind _returnvalue (`GameplayStatics.SpawnSoundAttached` "/Game/Audio/MetaSounds/SFX/MS_Assembly.MS_Assembly" (`self.DefaultSceneRoot`) "None" (0.0 0.0 0.0) (struct) "KeepRelativeOffset" false 1.0 1.0 0.0 null null))
    (set `self.AudioComponent` _returnvalue)
    (return true)
    (else
      (return _isminigamestartsuccess))))

(fn `UserConstructionScript`)