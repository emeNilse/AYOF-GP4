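; Cutting station interactable for cooking that animates a knife during its minigame and shows the held ingredient.
; Minigame start readies the knife animation; minigame finish stops it and passes the quality to the parent implementation.
; Inventory updates set the item mesh from the first slot's data table row, clearing it if none is found.
; Backup functions hold a debug-print check for Chopping-valid ingredients and an empty look-at text.
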(event `self.ReceiveBeginPlay`
  (add `self.MiniGameStart` (delegate `CallAnimation`))
  (add `/Game/Code/Core/Inventory/BP_InventorySystem.OnInventoryUpdated` (`self.BP_InventorySystem`) (delegate `UpdateDisplay`)))

(event `CallAnimation`
  (`/Game/Code/Interactables/BP_Knife.ReadyAnimation` (`self.Knife`)))

(event `UpdateDisplay`
  (`self.DisplayItem`))

(event `self.ReceiveTick`
  (params (DeltaSeconds :type "Float (single-precision)")))

(fn `CheckIngredientsBackup`
  (locals (isItemValid :type Boolean))
  (for _array_element (`/Game/Code/Core/Inventory/BP_InventorySystem.Content` (`self.BP_InventorySystem`))
    (bind _returnvalue (`|GetDataTableRow` "/Game/Code/Core/Inventory/ItemData.ItemData" (`.ItemID_2_9A35EB514A7E0F49F31B1696D16693F0` (break `/Game/Code/Core/Inventory/FSlotStruct` _array_element)))
      (:`then`
        (bind _output_get (set `local.isItemValid` (`|EnumEquality` (`.ValidMinigame` (break `ItemDataStruct` _returnvalue)) "Chopping")))
        (if _output_get
          (`KismetSystemLibrary.PrintString` "Valid Item")
          (else
            (`KismetSystemLibrary.PrintString` "Invalid item")))))))

(fn `DisplayItem`
  (bind _itemmesh (`self.ItemMesh`))
  (bind _returnvalue (`|GetDataTableRow` "/Game/Code/Core/Inventory/ItemData.ItemData" (`.ItemID_2_9A35EB514A7E0F49F31B1696D16693F0` (break `/Game/Code/Core/Inventory/FSlotStruct` (`|GetArrayItem` (`/Game/Code/Core/Inventory/BP_InventorySystem.Content` (`self.BP_InventorySystem`))))))
    (:`then`
      (`StaticMeshComponent.SetStaticMesh` _itemmesh (`.Mesh` (break `ItemAssetData` (`.ItemAssetData` (break `ItemDataStruct` _returnvalue))))))
    (:`RowNotFound`
      (`StaticMeshComponent.SetStaticMesh` _itemmesh null))))

(fn `LookAtBackup`
  (returns (Message :type Text))
  (return ""))

(fn `OnMinigameFinished`
  (params (Quality :type "Float (double-precision)"))
  (`/Game/Code/Interactables/BP_Knife.StopAnimation` (`self.Knife`))
  (`parent.OnMinigameFinished` Quality))

(fn `UserConstructionScript`)