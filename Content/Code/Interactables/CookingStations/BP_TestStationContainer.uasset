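; BP_TestStationContainer is a test cooking-station interactable with an inventory system component.
; On interaction, it shows its inventory as a container on the player controller's HUD.
; It then immediately spawns a hardcoded chopped meat actor at the inventory's drop location, prints a debug message, and completely removes the first slot's item.
; Its LookAt function returns an empty string.
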(event `/Game/Code/Core/Inventory/IInteractInterface.InteractWith`
  (params (PlayerCharacter :type "/Game/Code/Player/BP_Character Object Reference"))
  (bind _asbp_player_controller (cast `/Game/Code/Core/BP_PlayerController` (`GameplayStatics.GetPlayerController` 0)))
  (`/Game/Code/UI/UI_Inventory/W_PlayerHUD.ShowContainer` (`/Game/Code/Core/BP_PlayerController.HUD` _asbp_player_controller) (`self.BP_InventorySystem`))
  (`|SpawnActorFromClass` "/Game/Code/Interactables/ItemIngridients/BP_Meat_Chopped.BP_Meat_Chopped_C" (`KismetMathLibrary.MakeTransform` (`/Game/Code/Core/Inventory/BP_InventorySystem.GetDropLocation` (`self.BP_InventorySystem`))) "Undefined" "MultiplyWithRoot" null 0.0 null)
  (`KismetSystemLibrary.PrintString` "Spawned actor")
  (`/Game/Code/Core/Inventory/BP_InventorySystem.ServerRemove` (`self.BP_InventorySystem`) 0 true))

(fn `LookAt`
  (returns (Message :type Text))
  (return ""))

(fn `UserConstructionScript`)