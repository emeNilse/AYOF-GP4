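; Cooking station where a submitted dish ends the season.
; On IA_Interact it looks up each inventory item in the ItemData table: a Dish hides the inventories and calls EndSeason on the game mode, while other types trigger invalid-ingredient handling and leave the station.
; Inventory updates show the first item's mesh on the station, through a binding made every Tick.
; Actor-spawning branches are unconnected.
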(event `self.ReceiveTick`
  (params (DeltaSeconds :type "Float (single-precision)"))
  (add `/Game/Code/Core/Inventory/BP_InventorySystem.OnInventoryUpdated` (`self.BP_InventorySystem`) (delegate `DisplayItem`)))

(event `DisplayItem`
  (`self.DisplayDish`))

(event `CheckPlate`
  (bind _bp_inventorysystem (`self.BP_InventorySystem`))
  (if (`KismetArrayLibrary.Array_IsNotEmpty` (`/Game/Code/Core/Inventory/BP_InventorySystem.Content` _bp_inventorysystem))
    (for _array_element (`/Game/Code/Core/Inventory/BP_InventorySystem.Content` _bp_inventorysystem)
      (bind _returnvalue (`|GetDataTableRow` "/Game/Code/Core/Inventory/ItemData.ItemData" (`.ItemID_2_9A35EB514A7E0F49F31B1696D16693F0` (break `/Game/Code/Core/Inventory/FSlotStruct` _array_element)))
        (:`then`
          (if (`|EnumEquality` (`.ItemType` (break `ItemDataStruct` _returnvalue)) "Dish")
            (`self.HideInventories`)
            (bind _asayof_game_mode_base (cast `AyofGameModeBase` (`GameplayStatics.GetGameMode`)))
            (`AyofGameModeBase.EndSeason` _asayof_game_mode_base)
            (else
              (`self.OnInvalidIngredient`)
              (`self.LeaveStation`))))))))

(event `EnhancedInput|/Game/Code/Input/Actions/IA_Interact`
  (params (ActionValue :type Boolean) (ElapsedSeconds :type "Float (double-precision)") (TriggeredSeconds :type "Float (double-precision)") (InputAction :type "InputAction Object Reference" :default "/Game/Code/Input/Actions/IA_Interact.IA_Interact"))
  (:`Triggered`
    (`self.CheckPlate`)))

(fn `DisplayDish`
  (bind _returnvalue (`|GetDataTableRow` "/Game/Code/Core/Inventory/ItemData.ItemData" (`.ItemID_2_9A35EB514A7E0F49F31B1696D16693F0` (break `/Game/Code/Core/Inventory/FSlotStruct` (`|GetArrayItem` (`/Game/Code/Core/Inventory/BP_InventorySystem.Content` (`self.BP_InventorySystem`))))))
    (:`then`
      (`StaticMeshComponent.SetStaticMesh` (`self.Item`) (`.Mesh` (break `ItemAssetData` (`.ItemAssetData` (break `ItemDataStruct` _returnvalue))))))
    (:`RowNotFound`
      (`StaticMeshComponent.SetStaticMesh` (`self.Item`) null))))

(fn `OnInteract`
  (params (interactingPlayer :type "MyPlayerController Object Reference"))
  (locals (InventoryOpen :type Boolean)))

(fn `OnPossessed`
  (`parent.OnPossessed`))

(fn `OnUnPossessed`
  (`parent.OnUnPossessed`))

(fn `TryStartMinigame`
  (returns (isMinigameStartSuccess :type Boolean))
  (bind _isminigamestartsuccess (`parent.TryStartMinigame`))
  (return _isminigamestartsuccess))

(fn `UserConstructionScript`)