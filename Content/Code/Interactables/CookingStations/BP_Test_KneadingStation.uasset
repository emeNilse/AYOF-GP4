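; Test Blueprint for a kneading cooking station, holding backup versions of its ingredient check and look-at functions.
; CheckIngredientsBackup loops over the inventory system's content, looks up each item in the ItemData table and tests whether its valid minigame is Kneading.
; Each found row overwrites a single validity flag and prints a debug message, so the last one wins.
; LookAtBackup returns an empty string, and the construction script is empty.
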(fn `CheckIngredientsBackup`
  (for _array_element (`/Game/Code/Core/Inventory/BP_InventorySystem.Content` (`self.BP_InventorySystem`))
    (bind _returnvalue (`|GetDataTableRow` "/Game/Code/Core/Inventory/ItemData.ItemData" (`.ItemID_2_9A35EB514A7E0F49F31B1696D16693F0` (break `/Game/Code/Core/Inventory/FSlotStruct` _array_element)))
      (:`then`
        (if (`|EnumEquality` (`.ValidMinigame` (break `ItemDataStruct` _returnvalue)) "Kneading")
          (set `self.ItemIsValidBackup` true)
          (`KismetSystemLibrary.PrintString` "Valid Item")
          (else
            (set `self.ItemIsValidBackup` false)
            (`KismetSystemLibrary.PrintString` "Invalid item")))))))

(fn `LookAtBackup`
  (returns (Message :type Text))
  (return ""))

(fn `UserConstructionScript`)