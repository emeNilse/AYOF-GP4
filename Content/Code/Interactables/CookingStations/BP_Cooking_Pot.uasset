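; Cooking pot station that gives visual and audio feedback for its inventory and cooking minigame.
; Inventory updates show a Kalops filler mesh when any item has a positive quantity and clear it otherwise.
; Minigame start readies the Spoon animation and spawns an attached stovetop MetaSound.
; Spoon animation events fire the sound's stir trigger, and minigame finish stops both before handing the quality to the parent class.
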(event `self.ReceiveBeginPlay`
  (add `self.MiniGameStart` (delegate `CallAnimation`))
  (`self.SafeBindToSpoonAnimation`)
  (add `/Game/Code/Core/Inventory/BP_InventorySystem.OnInventoryUpdated` (`self.BP_InventorySystem`) (delegate `UpdateDisplay`)))

(event `UpdateDisplay`
  (`self.CheckIfNotEmpty`))

(event `CallAnimation`
  (`/Game/Code/Interactables/BP_Spoon_CookingPot.ReadyAnimation` (`self.Spoon`))
  (bind _returnvalue (`GameplayStatics.SpawnSoundAttached` "/Game/Audio/MetaSounds/SFX/MS_Stovetop.MS_Stovetop" (`self.StaticMesh`) "None" (0.0 0.0 0.0) (struct) "KeepRelativeOffset" false 1.0 1.0 0.0 null null))
  (set `self.AudioComponent` _returnvalue))

(event `self.ReceiveTick`
  (params (DeltaSeconds :type "Float (single-precision)"))
  (`parent.ReceiveTick` DeltaSeconds))

(fn `CheckIfNotEmpty`
  (`|ExecutionSequence`
    (:`then_0`
      (set `self.LocalCounter` 0)
      (for _array_element (`/Game/Code/Core/Inventory/BP_InventorySystem.Content` (`self.BP_InventorySystem`))
        (if (> (`.Quantity_5_614ED38643097AB082B4D6BD820F5592` (break `/Game/Code/Core/Inventory/FSlotStruct` _array_element)) 0)
          (`/Engine/EditorBlueprintResources/StandardMacros.IncrementInt` (`self.LocalCounter`)))))
    (:`then_1`
      (if (> (`self.LocalCounter`) 0)
        (`self.DisplayItem`)
        (else
          (`self.RemoveDisplayedItem`))))))

(fn `DisplayItem`
  (if (not (`self.MeshDisplayed`))
    (bind _returnvalue (`StaticMeshComponent.SetStaticMesh` (`self.Filler`) "/Game/Art/1-Assets/Ingredients/PotAndBowlFiller/SM_KalopsInPot.SM_KalopsInPot"))
    (set `self.MeshDisplayed` _returnvalue)))

(fn `OnAnimationTriggered`
  (bind _audiocomponent (`self.AudioComponent`))
  (`/Engine/EditorBlueprintResources/StandardMacros.IsValid` _audiocomponent
    (:`Is Valid`
      (`AudioParameterControllerInterface.SetTriggerParameter` _audiocomponent "Stir"))))

(fn `OnMinigameFinished`
  (params (Quality :type "Float (double-precision)"))
  (`/Game/Code/Interactables/BP_Spoon_CookingPot.StopAnimation` (`self.Spoon`))
  (`AudioParameterControllerInterface.SetTriggerParameter` (`self.AudioComponent`) "StopAll")
  (`parent.OnMinigameFinished` Quality))

(fn `RemoveDisplayedItem`
  (`StaticMeshComponent.SetStaticMesh` (`self.Filler`) null)
  (set `self.MeshDisplayed` false))

(fn `SafeBindToSpoonAnimation`
  (bind _spoon (`self.Spoon`))
  (`/Engine/EditorBlueprintResources/StandardMacros.IsValid` _spoon
    (:`Is Valid`
      (add `/Game/Code/Interactables/BP_Spoon_CookingPot.AnimationTriggered` _spoon (`|CreateDelegate` :!event `OnAnimationTriggered`)))))

(fn `UserConstructionScript`
  (`parent.UserConstructionScript`))