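; Base possessable cooking station that turns deposited ingredients into crafted items through a minigame.
; Possession opens the station inventory, and Interact validates its contents against the optional minigame-type and recipe DataTable checks before spawning the minigame.
; On completion it spawns the result with the quality score, clears ingredients and returns control to the character.
; Dialogue gives feedback; child Blueprints can override Interact for other behavior.
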(event `self.ReceiveTick`
  (params (DeltaSeconds :type "Float (single-precision)")))

(event `EnhancedInput|/Game/Code/Input/Actions/IA_Interact`
  (params (ActionValue :type Boolean) (ElapsedSeconds :type "Float (double-precision)") (TriggeredSeconds :type "Float (double-precision)") (InputAction :type "InputAction Object Reference" :default "/Game/Code/Input/Actions/IA_Interact.IA_Interact"))
  ; if you want to do something other than start a minigame, on a bp that inherrits from this one, override this input action
  (:`Started`
    (`self.TryStartMinigame`)))

(event `self.ReceivePossessed`
  (params (NewController :type "Controller Object Reference"))
  ; Default OnPossessed just displays possession dialogue and opens the inventory ui
  (`self.OnPossessed`))

(event `self.ReceiveUnpossessed`
  (params (OldController :type "Controller Object Reference"))
  ; default OnUnPossessed displays optional dialogue for unpossession, and closes the inventory ui if it is still open
  (`self.OnUnPossessed`))

(fn `CheckIngredients`
  (returns (areAllIngredientsValid :type Boolean) (ingredientsFound :type Integer))
  (locals (currentItemValid :type Boolean :default false) (InventoryContainsItems :type Boolean) (currentSlotItemId :type Name) (currenSlotStackSize :type Integer) (PossibleRecipes :type "Map of Name to Object Object Reference") (currentRecipeKey :type Name) (numIngredients :type Integer))
  (set `local.numIngredients` 0)
  (for _array_element (`/Game/Code/Core/Inventory/BP_InventorySystem.Content` (`self.BP_InventorySystem`))
    (`|ExecutionSequence`
      (:`then_0`
        (bind (_itemid _quantity) (break `/Game/Code/Core/Inventory/FSlotStruct` _array_element))
        ; current item slot data saved as local variables for better readability
        (set `local.currentSlotItemId` _itemid)
        (set `local.currenSlotStackSize` _quantity))
      (:`then_1`
        ; if slot contains an item, mark that we found an item to process, and check if it is valid
        (if (> (`local.currenSlotStackSize`) 0)
          (`/Engine/EditorBlueprintResources/StandardMacros.IncrementInt` (`local.numIngredients`)
            (:`  `
              (`|ExecutionSequence`
                (:`then_0`
                  (set `local.InventoryContainsItems` true)
                  ; check if an item is a match for our minigame
                  (if (`self.bMatchToMinigame`)
                    (bind _returnvalue (`|GetDataTableRow` "/Game/Code/Core/Inventory/ItemData.ItemData" (`local.currentSlotItemId`))
                      (:`then`
                        (set `local.currentItemValid` (`|EnumEquality` (`.ValidMinigame` (break `ItemDataStruct` _returnvalue)) (`.MinigameType` (defaults `Object` (`self.MiniGame`)))))))
                    (else
                      (set `local.currentItemValid` true))))
                (:`then_1`
                  ; break if invalid item found
                  (if (not (`local.currentItemValid`))
                    (`KismetSystemLibrary.PrintString` "invalid item found breaking early" true true (struct :`R` 1.0 :`G` 0.01231 :`A` 1.0) 2.0 "cookstationIngredientCheck")
                    (break))))))))))
  ; after loop, if items were found return whether items were found and if they were all valid
  (if (`local.InventoryContainsItems`)
    (return (`local.currentItemValid`) (`local.numIngredients`))
    (else
      (return false 0))))

(fn `DeleteUsedIngredients`
  (for (_array_element _array_index) (`/Game/Code/Core/Inventory/BP_InventorySystem.Content` (`self.BP_InventorySystem`))
    ; debug check what's in the inventory
    (`/Game/Code/Core/Inventory/BP_InventorySystem.ServerRemove` (`self.BP_InventorySystem`) _array_index true)
    (`KismetSystemLibrary.PrintString` (`KismetStringLibrary.Concat_StrStr` "After server remove completely we found " (`KismetStringLibrary.Conv_NameToString` (`.ItemID_2_9A35EB514A7E0F49F31B1696D16693F0` (break `/Game/Code/Core/Inventory/FSlotStruct` _array_element))) " in " (`KismetSystemLibrary.GetDisplayName` self) "'s inventory"))))

(fn `FindRecipe`
  (params (CurrentIngredientId :type Name) (ActualNumInventoryItems :type Integer))
  (returns (isRecipeFound :type Boolean) (FoundRecipeOutput :type "ItemDataStruct Structure"))
  (locals (currentRecipeIngredients :type "Array of ItemDataStruct Structure") (currentRecipeOutput :type "ItemDataStruct Structure") (PossibleRecipes :type "Array of Name") (currentRecipe :type Name) (currentRecipeIngredient :type Name) (Found :type Boolean) (currentInventoryIngredient :type Name))
  (bind _found (`local.Found`))
  (bind _outrownames (`DataTableFunctionLibrary.GetDataTableRowNames` (`self.RecipeDataTable`)))
  (for _array_element _outrownames
    (`|ExecutionSequence`
      (:`then_0`
        ; get current recipe ingredients and outputs as local variables
        (bind _output_get (set `local.currentRecipe` _array_element))
        (bind _returnvalue (`|GetDataTableRow` (`self.RecipeDataTable`) _output_get)
          (:`then`
            (bind (_recipe_ingredients _recipe_result) (break `Recipe` (break `/Game/Code/Core/Inventory/FSlot_Recipe_Struct` _returnvalue)))
            (set `local.currentRecipeIngredients` _recipe_ingredients)
            (set `local.currentRecipeOutput` _recipe_result))
          (:`RowNotFound`
            (`KismetSystemLibrary.PrintString` "this shouldn't be possible to fire" true true (struct :`R` 1.0 :`B` 0.033888 :`A` 1.0) 2.0 "bp_CookingStation:FindRecipe"))))
      (:`then_1`
        ; if there are more or less ingredients in station than are in the recipe, check next recipe
        (if (== (`KismetArrayLibrary.Array_Length` (`local.currentRecipeIngredients`)) (`local.ActualNumInventoryItems`))
          ; check if contents match a recipe
          (for _array_element_2 (`local.currentRecipeIngredients`)
            (`|ExecutionSequence`
              (:`then_0`
                ; initialize loop variables
                (set `local.currentRecipeIngredient` (`.ID` (break `ItemDataStruct` _array_element_2)))
                (set `local.Found` false))
              (:`then_1`
                ; are any of the ingredients in the station a match to the current recipe ingredient
                (for _array_element_3 (`/Game/Code/Core/Inventory/BP_InventorySystem.Content` (`self.BP_InventorySystem`))
                  (bind _output_get_2 (set `local.currentInventoryIngredient` (`.ItemID_2_9A35EB514A7E0F49F31B1696D16693F0` (break `/Game/Code/Core/Inventory/FSlotStruct` _array_element_3))))
                  (if (== _output_get_2 (`local.currentRecipeIngredient`))
                    (set `local.Found` true)
                    (break)))
                (if (not (`local.Found`))
                  (break)))))
          (if _found
            (return _found (`local.currentRecipeOutput`)))
          (else
            (set `local.Found` false))))))
  (return false))

(fn `HideInventories`
  (if (`self.bIsContainerUiVisible`)
    (bind _asbp_player_controller (cast `/Game/Code/Core/BP_PlayerController` (`GameplayStatics.GetPlayerController` 0)))
    (`/Game/Code/UI/UI_Inventory/W_PlayerHUD.HideContainer` (`/Game/Code/Core/BP_PlayerController.HUD` _asbp_player_controller))
    (set `self.bIsContainerUiVisible` false)))

(fn `LeaveStation`
  (bind _asmy_player_controller (cast `MyPlayerController` (`GameplayStatics.GetPlayerController` 0)))
  (`MyPlayerController.SwitchToCharacter` _asmy_player_controller))

(fn `LookAt`
  (returns (Message :type Text) (SM :type "StaticMeshComponent Object Reference"))
  (return (`KismetTextLibrary.Conv_NameToText` (`self.Name`)) null))

(fn `NoIngredientsFeedback`
  (`DialogueEventComponent.StartDialogueEvent` (`self.BP_DialogueComponent`) (`self.NoIngredients`) false)
  (`KismetSystemLibrary.PrintString` "TODO: replace this node witha call to a sound effect later"))

(fn `OnInvalidIngredient`
  (`DialogueEventComponent.StartDialogueEvent` (`self.BP_DialogueComponent`) (`self.InvalidIngredient`) false)
  (`KismetSystemLibrary.PrintString` "TODO: INVALID COOKING INGREDIENT SUBMITTED replace this with sound or visual effects"))

(fn `OnInventoryButtonPressed`
  (params (Success :type Boolean) (wasSendingItemToStation :type Boolean)))

(fn `OnMinigameFinished`
  (params (Quality :type "Float (double-precision)"))
  (bind _returnvalue (>= (`local.Quality`) 1.0))
  (bind _spawnedatlocation (`self.SpawnCraftedItem` Quality))
  (`self.PlayItemDropSound` _spawnedatlocation)
  (`self.DeleteUsedIngredients`)
  (`self.LeaveStation`)
  ; playerfeedback on success or fail
  (if (`self.bShowDialogueOnMinigameResult`)
    (`DialogueEventComponent.StartDialogueEvent` (`self.BP_DialogueComponent`) (`KismetMathLibrary.SelectName` (`self.SuccessfulCooking`) (`self.FailedCooking`) _returnvalue) false)
    (`KismetSystemLibrary.PrintString` "TODO: replace this debug with sound or visual effects for a SUCCESS cooking result" :!label _label)
    (elif _returnvalue
      (goto _label)
      (else
        (`KismetSystemLibrary.PrintString` "TODO: replace this debug with sound or visual effects for a FAIL cooking result")))))

(fn `OnPossessed`
  (if (`self.bShowDialogueOnPossess`)
    (`DialogueEventComponent.StartDialogueEvent` (`self.BP_DialogueComponent`) (`self.PossessedDialogue`) false))
  (`self.ShowInventories`))

(fn `OnUnPossessed`
  (if (`self.bShowDialogueOnUnPossess`)
    (`DialogueEventComponent.StartDialogueEvent` (`self.BP_DialogueComponent`) (`self.UnPossessedDialogue`) false))
  (`self.HideInventories`))

(fn `OnUnPossessed_0`)

(fn `PlayItemDropSound`
  (params (Location :type "Vector Structure"))
  (bind _returnvalue (`GameplayStatics.SpawnSoundAtLocation` "/Game/Audio/MetaSounds/SFX/MS_BaseIngredientSounds.MS_BaseIngredientSounds" Location (struct) 1.0 1.0 0.0 null null))
  (`AudioParameterControllerInterface.SetTriggerParameter` _returnvalue "OnSetDown"))

(fn `ShowInventories`
  (bind _asbp_player_controller (cast `/Game/Code/Core/BP_PlayerController` (`GameplayStatics.GetPlayerController` 0)))
  (bind _hud (`/Game/Code/Core/BP_PlayerController.HUD` _asbp_player_controller))
  (add `/Game/Code/UI/UI_Inventory/W_PlayerHUD.InventoryButtonResult` _hud (`|CreateDelegate` :!event `OnInventoryButtonPressed`))
  (`/Game/Code/UI/UI_Inventory/W_PlayerHUD.ShowContainer` _hud (`self.BP_InventorySystem`))
  (set `self.bIsContainerUiVisible` true))

(fn `SpawnCraftedItem`
  (params (newQuality :type "Float (double-precision)"))
  (returns (SpawnedAtLocation :type "Vector Structure"))
  (locals (ItemClass :type "Actor Class Reference") (SpawnLocation :type "Vector Structure" :default (0.0 0.0 0.0)))
  (bind (_reciperesultdata_id _reciperesultdata_itemtype _reciperesultdata_itemquality _reciperesultdata_itemgrade _reciperesultdata_validminigame _reciperesultdata_itemassetdata) (break `ItemDataStruct` (`self.RecipeResultData`)))
  (bind (_returnvalue_x _returnvalue_y _returnvalue_z) (`KismetMathLibrary.BreakVector` (`self.K2_GetActorLocation` (`ActorComponent.GetOwner` (`self.StaticMesh`)))))
  (if (`self.bUseRecipes`)
    ; if using recipes get recipe output class
    (set `local.ItemClass` (`.ItemClass` (break `ItemAssetData` _reciperesultdata_itemassetdata)))
    (else
      ; if not using recipes get output class from single input item
      (set `local.ItemClass` (`.ItemClass` (break `ItemAssetData` (`.Item Asset Data` (`/Game/Code/Core/Inventory/BP_InventorySystem.GetSlotItem` (`self.BP_InventorySystem`))))))))
  (set `local.SpawnLocation` (`KismetMathLibrary.MakeVector` (- _returnvalue_x (`self.SpawnX`)) (- _returnvalue_y (`self.SpawnY`)) (- _returnvalue_z (`self.SpawnZ`))))
  (bind _returnvalue (`|SpawnActorFromClass` (`local.ItemClass`) (`KismetMathLibrary.MakeTransform` (`local.SpawnLocation`)) "Undefined" "MultiplyWithRoot" null null))
  (`NiagaraFunctionLibrary.SpawnSystemAtLocation` "/Game/Art/VFX/Sparks_Once.Sparks_Once" (`local.SpawnLocation`))
  (`KismetSystemLibrary.PrintText` (`|FormatText` "Spawned an {item} at {location}" (`KismetSystemLibrary.GetClassDisplayName` (`local.ItemClass`)) (`KismetStringLibrary.Conv_VectorToString` (`local.SpawnLocation`))) true true (struct :`G` 0.66 :`B` 1.0 :`A` 1.0) 2.0 "CookingStationItemSpawn")
  ; I think if we can set the item class in the item data struct to something with quality, we shouldn't need to do this cast
  (bind _asbp_base_item (cast `/Game/Code/Interactables/ItemIngridients/BP_BaseItem` _returnvalue))
  (set `/Game/Code/Interactables/ItemIngridients/BP_BaseItem.QualityBP` (`local.newQuality`) _asbp_base_item)
  (return (`local.SpawnLocation`)))

(fn `SpawnMinigame`
  (bind _returnvalue (`|SpawnActorFromClass` (`self.MiniGame`) (`KismetMathLibrary.MakeTransform` (`SceneComponent.K2_GetComponentLocation` (`self.Camera`))) "Undefined" "MultiplyWithRoot" null null))
  (add `/Game/Code/MiniGames/BP_MG.OnMinigameCompleted` _returnvalue (`|CreateDelegate` :!event `OnMinigameFinished`)))

(fn `TryStartMinigame`
  (returns (isMinigameStartSuccess :type Boolean))
  (`|ExecutionSequence`
    (:`then_0`
      (bind (_areallingredientsvalid _ingredientsfound) (`self.CheckIngredients`)))
    (:`then_1`
      (`/Engine/EditorBlueprintResources/StandardMacros.CompareInt` _ingredientsfound
        (:`>`
          ; if ingredients were found
          (if _areallingredientsvalid
            (if (`self.bUseRecipes`)
              ; if we're using recipes save the output for later
              (bind (_isrecipefound _foundrecipeoutput) (`self.FindRecipe` "None" _ingredientsfound))
              (if _isrecipefound
                (set `self.RecipeResultData` _foundrecipeoutput)
                (else
                  (`self.OnInvalidIngredient`)
                  (return false))))
            (`self.HideInventories`)
            (`self.SpawnMinigame`)
            (`self.MiniGameStart`)
            (return true)
            (else
              (`self.OnInvalidIngredient`)
              (return false))))
        (:`==`
          _)
        (:`<`
          _))
      ; NoIngredients found
      (`self.NoIngredientsFeedback`)
      (return false))))

(fn `UserConstructionScript`)