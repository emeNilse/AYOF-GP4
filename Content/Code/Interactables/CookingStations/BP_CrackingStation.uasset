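; Possessable cooking station that runs a minigame on ingredients placed in its inventory, which interacting opens on the HUD.
; On possession it checks items against the ItemData table for the Chopping minigame; the last slot checked decides validity.
; If valid, it spawns the minigame, cast to BP_MG_Cutting, whose completion spawns the slot item's class and removes it from inventory.
; Quality is unused, ChangeIngredientStatus is unfinished, and Tick prints debug output.
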(event `self.ReceiveTick`
  (params (DeltaSeconds :type "Float (single-precision)"))
  (for _array_element (`/Game/Code/Core/Inventory/BP_InventorySystem.Content` (`self.BP_InventorySystem`))
    (bind _returnvalue (`|GetDataTableRow` "/Game/Code/Core/Inventory/ItemData.ItemData" (`.ItemID_2_9A35EB514A7E0F49F31B1696D16693F0` (break `/Game/Code/Core/Inventory/FSlotStruct` _array_element)))
      (:`then`
        (`KismetSystemLibrary.PrintString` (`|GetEnumeratorNameAsString` (`.ItemQuality` (break `ItemDataStruct` _returnvalue))))
        (`KismetSystemLibrary.PrintString` (`KismetStringLibrary.Conv_IntToString` (`self.Iterations`)))))))

(event `self.ReceivePossessed`
  (params (NewController :type "Controller Object Reference"))
  (`|ExecutionSequence`
    (:`then_0`
      (`self.CheckIngredients`))
    (:`then_1`
      ; If Ingridient check returns valid Spawn minigame
      ;;[1 0.7424 0 0.5] TODO:: If return false unpossess character
      (if (`self.ItemIsValid`)
        (bind _returnvalue (`|SpawnActorFromClass` (`self.MiniGame`) (`KismetMathLibrary.MakeTransform` (`SceneComponent.K2_GetComponentLocation` (`self.Camera`))) "Undefined" "MultiplyWithRoot" null null))
        (bind _asbp_mg_cutting (cast `/Game/Code/MiniGames/BP_MG_Cutting` _returnvalue))
        (add `/Game/Code/MiniGames/BP_MG_Cutting.OnMinigameCompleted` _asbp_mg_cutting (delegate `OnFinished`))))))

(event `OnFinished`
  (params (Quality :type "Float (double-precision)"))
  (bind (_id _item_type _item_quality _item_grade _valid_minigame _item_asset_data) (`/Game/Code/Core/Inventory/BP_InventorySystem.GetSlotItem` (`self.BP_InventorySystem`)))
  (bind (_returnvalue_x _returnvalue_y _returnvalue_z) (`KismetMathLibrary.BreakVector` (`self.K2_GetActorLocation` (`ActorComponent.GetOwner` (`self.Cube`)))))
  ; Remove item from station inventory and spawn items result ingridient
  (if (`self.ItemIsValid`)
    (`|SpawnActorFromClass` (`.ItemClass` (break `ItemAssetData` _item_asset_data)) (`KismetMathLibrary.MakeTransform` (`KismetMathLibrary.MakeVector` _returnvalue_x _returnvalue_y (- _returnvalue_z 20.0))) "Undefined" "MultiplyWithRoot" null null)
    (`KismetSystemLibrary.PrintString` (`KismetSystemLibrary.GetClassDisplayName` (`.ItemClass` (break `ItemAssetData` _item_asset_data))))
    (`/Game/Code/Core/Inventory/BP_InventorySystem.ServerRemove` (`self.BP_InventorySystem`) 0 true)))

(event `self.InteractWith`
  (params (PlayerCharacter :type "/Game/Code/Player/BP_Character Object Reference"))
  (bind _asbp_player_controller (cast `/Game/Code/Core/BP_PlayerController` (`GameplayStatics.GetPlayerController` 0)))
  (`/Game/Code/UI/UI_Inventory/W_PlayerHUD.ShowContainer` (`/Game/Code/Core/BP_PlayerController.HUD` _asbp_player_controller) (`self.BP_InventorySystem`)))

(fn `ChangeIngredientStatus`
  (locals (NewLocalVar :type "EItemQuality Enum") (OutRow :type "ItemDataStruct Structure") (Quality :type "EItemQuality Enum") (Validgame :type "EValidMinigame Enum") (NewLocalVar_0 :type "EValidMinigame Enum"))
  (for _array_element (`/Game/Code/Core/Inventory/BP_InventorySystem.Content` (`self.BP_InventorySystem`))
    (bind _returnvalue (`|GetDataTableRow` "/Game/Code/Core/Inventory/ItemData.ItemData" (`.ItemID_2_9A35EB514A7E0F49F31B1696D16693F0` (break `/Game/Code/Core/Inventory/FSlotStruct` _array_element)))
      (:`then`
        (if (`|EnumEquality` (`.ValidMinigame` (break `ItemDataStruct` _returnvalue)) "Chopping")
          _)))))

(fn `CheckIngredients`
  (for _array_element (`/Game/Code/Core/Inventory/BP_InventorySystem.Content` (`self.BP_InventorySystem`))
    (bind _itemid (break `/Game/Code/Core/Inventory/FSlotStruct` _array_element))
    (bind _returnvalue (`|GetDataTableRow` "/Game/Code/Core/Inventory/ItemData.ItemData" _itemid)
      (:`then`
        (if (!= _itemid "None")
          (if (`|EnumEquality` (`.ValidMinigame` (break `ItemDataStruct` _returnvalue)) "Chopping")
            (set `self.ItemIsValid` true)
            (`KismetSystemLibrary.PrintString` "Valid Item")
            (set `self.Iterations` (+ (`self.Iterations`) 1))
            (else
              (set `self.ItemIsValid` false :!label _label)
              (`KismetSystemLibrary.PrintString` "Invalid item")))
          (else
            (`KismetSystemLibrary.PrintString` "Slot is null")
            (goto _label)))))))

(fn `LookAt`
  (returns (Message :type Text))
  (return ""))

(fn `UserConstructionScript`)