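; BP_SummerOven is a possessable cooking station that turns Batter into CakeBase.
; On jump input release, it scans the player's inventory for batter and spawns the configured minigame at the camera.
; A kneading minigame awards CakeBase through its completion callback, ignoring quality; other outcomes of the cast award it immediately.
; RemoveItem only prints item IDs, since its removal call is disconnected, so Batter stays in the inventory.
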(event `self.ReceiveBeginPlay`)

(event `self.ReceivePossessed`
  (params (NewController :type "Controller Object Reference"))
  (set `self.New Controller` NewController))

(event `self.ReceiveUnpossessed`
  (params (OldController :type "Controller Object Reference")))

(event `EnhancedInput|/Game/Code/Input/Actions/IA_Jump`
  (params (ActionValue :type Boolean) (ElapsedSeconds :type "Float (double-precision)") (TriggeredSeconds :type "Float (double-precision)") (InputAction :type "InputAction Object Reference" :default "/Game/Code/Input/Actions/IA_Jump.IA_Jump"))
  (:`Completed`
    (bind _asmy_player_controller (cast `MyPlayerController` (`GameplayStatics.GetPlayerController` 0)))
    (for _array_element (`/Game/Code/Core/Inventory/BP_InventorySystem.Content` (`self.GetComponentByClass` (`MyPlayerController.CharacterPawn` _asmy_player_controller) "/Game/Code/Core/Inventory/BP_InventorySystem.BP_InventorySystem_C"))
      (if (== (`.ItemID_2_9A35EB514A7E0F49F31B1696D16693F0` (break `/Game/Code/Core/Inventory/FSlotStruct` _array_element)) (`self.BatterID`))
        (bind _returnvalue (`|SpawnActorFromClass` (`self.Minigame`) (`KismetMathLibrary.MakeTransform` (`SceneComponent.K2_GetComponentLocation` (`self.Camera`))) "Undefined" "MultiplyWithRoot" null null))
        (bind _asbp_mg_kneading (cast `/Game/Code/MiniGames/BP_MG_Kneading` _returnvalue)
          (:`then`
            (add `/Game/Code/MiniGames/BP_MG_Kneading.OnMinigameCompleted` _asbp_mg_kneading (delegate `OnFirstFinished`)))
          (:`CastFailed`
            (`self.AddItem` "CakeBase" :!label _label)
            (`self.RemoveItem` "Batter")))))))

(event `OnFirstFinished`
  (params (Quality :type "Float (double-precision)"))
  (goto _label))

(fn `AddItem`
  (params (ItemID :type Name))
  (bind _asmy_player_controller (cast `MyPlayerController` (`GameplayStatics.GetPlayerController` 0)))
  (`/Game/Code/Core/Inventory/BP_InventorySystem.AddToInventory` (`self.GetComponentByClass` (`MyPlayerController.CharacterPawn` _asmy_player_controller) "/Game/Code/Core/Inventory/BP_InventorySystem.BP_InventorySystem_C") ItemID 1))

(fn `RemoveItem`
  (params (ItemID :type Name))
  (bind _asmy_player_controller (cast `MyPlayerController` (`self.New Controller`))
    (:`then`
      (for (_array_element _array_index) (`/Game/Code/Core/Inventory/BP_InventorySystem.Content` (`self.GetComponentByClass` (`MyPlayerController.CharacterPawn` _asmy_player_controller) "/Game/Code/Core/Inventory/BP_InventorySystem.BP_InventorySystem_C"))
        (bind _itemid (break `/Game/Code/Core/Inventory/FSlotStruct` _array_element))
        (`KismetSystemLibrary.PrintString` (`KismetStringLibrary.Conv_NameToString` _itemid))
        (if (== _itemid ItemID)
          _)))
    (:`CastFailed`
      (`KismetSystemLibrary.PrintString` "Cast Failed!"))))

(fn `UserConstructionScript`)