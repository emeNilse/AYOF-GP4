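; BP_Trash_Station is a possessable cooking station that discards the player's ingredients.
; Pressing Interact finishes the minigame with zero quality, which deletes the used ingredients and leaves the station.
; Possession opens the lid and unpossession closes it if open, through a FlipFlop that plays or reverses a timeline rotating the Pivot.
; The trash sound plays as opening starts and when closing finishes.
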(event `Open&Close`
  (bind _isa (`/Engine/EditorBlueprintResources/StandardMacros.FlipFlop`)
    (:`A`
      (`GameplayStatics.SpawnSoundAttached` "/Game/Audio/MetaSounds/SFX/MS_Trash.MS_Trash" (`self.Pivot`) "None" (0.0 0.0 0.0) (struct) "KeepRelativeOffset" false 1.0 1.0 0.0 null null)
      (bind (_direction _newtrack_0) (`Timeline|LidOpen` :!label _label)
        (:`Update`
          (set `self.Is A` _isa)
          (`SceneComponent.K2_SetRelativeRotation` (`self.Pivot`) (`KismetMathLibrary.MakeRotator` (`KismetMathLibrary.Lerp` 0.0 -90.0 _newtrack_0) 0.0 90.0) false false))
        (:`Finished`
          (if (not (`self.Is A`))
            (`GameplayStatics.SpawnSoundAttached` "/Game/Audio/MetaSounds/SFX/MS_Trash.MS_Trash" (`self.Pivot`) "None" (0.0 0.0 0.0) (struct) "KeepRelativeOffset" false 1.0 1.0 0.0 null null)))))
    (:`B`
      (goto _label :!via `Reverse`))))

(event `EnhancedInput|/Game/Code/Input/Actions/IA_Interact`
  (params (ActionValue :type Boolean) (ElapsedSeconds :type "Float (double-precision)") (TriggeredSeconds :type "Float (double-precision)") (InputAction :type "InputAction Object Reference" :default "/Game/Code/Input/Actions/IA_Interact.IA_Interact"))
  (:`Started`
    (`self.OnMinigameFinished` 0.0)))

(fn `OnMinigameFinished`
  (params (Quality :type "Float (double-precision)"))
  (`self.DeleteUsedIngredients`)
  (`self.LeaveStation`))

(fn `OnPossessed`
  (`self.Open&Close`)
  (`parent.OnPossessed`))

(fn `OnUnPossessed`
  (if (`self.Is A`)
    (`self.Open&Close`))
  (`parent.OnUnPossessed`))

(fn `TryStartMinigame`
  (returns (isMinigameStartSuccess :type Boolean))
  (bind _isminigamestartsuccess (`parent.TryStartMinigame`))
  (return _isminigamestartsuccess))

(fn `UserConstructionScript`
  (`parent.UserConstructionScript`))