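; Oven cooking station that extends a parent station class with an animated door and a display of its inventory item.
; Possess, unpossess, minigame-start and leave overrides toggle the door through a FlipFlop-driven timeline and MetaSound triggers.
; Inventory updates, rebound every Tick, refresh the item mesh from a data table.
; OnFinished spawns the slot item's class, removes it and returns to the character, but its minigame binding is in disconnected logic.
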(event `self.ReceiveBeginPlay`)

(event `self.ReceiveTick`
  (params (DeltaSeconds :type "Float (single-precision)"))
  (`parent.ReceiveTick` DeltaSeconds)
  (add `/Game/Code/Core/Inventory/BP_InventorySystem.OnInventoryUpdated` (`self.BP_InventorySystem`) (delegate `CallDisplayItem`)))

(event `CallDisplayItem`
  (`self.DisplayItem`))

(event `Open&Close`
  (bind _returnvalue (`GameplayStatics.SpawnSoundAtLocation` "/Game/Audio/MetaSounds/SFX/MS_Oven.MS_Oven" (`SceneComponent.K2_GetComponentLocation` (`self.Door`)) (struct) 1.0 1.0 0.0 null null))
  (bind _isa (`/Engine/EditorBlueprintResources/StandardMacros.FlipFlop`)
    (:`A`
      (`AudioParameterControllerInterface.SetTriggerParameter` _returnvalue "Open")
      (bind (_direction _newtrack_0) (`Timeline|DoorTimeLine` :!label _label)
        (:`Update`
          (set `self.Is A` _isa)
          (`SceneComponent.K2_SetRelativeRotation` (`self.Door`) (`KismetMathLibrary.MakeRotator` (`KismetMathLibrary.Lerp` 0.0 -90.0 _newtrack_0) 0.0 -90.0) false false))))
    (:`B`
      (`AudioParameterControllerInterface.SetTriggerParameter` _returnvalue "Close")
      (goto _label :!via `Reverse`))))

(event `OnFinished`
  (params (Quality :type "Float (double-precision)"))
  (bind (_returnvalue_x _returnvalue_y _returnvalue_z) (`KismetMathLibrary.BreakVector` (`self.K2_GetActorLocation` (`ActorComponent.GetOwner` (`self.StaticMesh`)))))
  (`|SpawnActorFromClass` (`.ItemClass` (break `ItemAssetData` (`.Item Asset Data` (`/Game/Code/Core/Inventory/BP_InventorySystem.GetSlotItem` (`self.BP_InventorySystem`))))) (`KismetMathLibrary.MakeTransform` (`KismetMathLibrary.MakeVector` _returnvalue_x _returnvalue_y (- _returnvalue_z 20.0))) "Undefined" "MultiplyWithRoot" null null)
  (`/Game/Code/Core/Inventory/BP_InventorySystem.ServerRemove` (`self.BP_InventorySystem`) 0 false)
  (bind _asbp_player_controller (cast `/Game/Code/Core/BP_PlayerController` (`GameplayStatics.GetPlayerController` 0)))
  (`MyPlayerController.SwitchToCharacter` _asbp_player_controller))

(fn `DisplayItem`
  (bind _returnvalue (`|GetDataTableRow` "/Game/Code/Core/Inventory/ItemData.ItemData" (`.ItemID_2_9A35EB514A7E0F49F31B1696D16693F0` (break `/Game/Code/Core/Inventory/FSlotStruct` (`|GetArrayItem` (`/Game/Code/Core/Inventory/BP_InventorySystem.Content` (`self.BP_InventorySystem`))))))
    (:`then`
      (`StaticMeshComponent.SetStaticMesh` (`self.ItemMesh`) (`.Mesh` (break `ItemAssetData` (`.ItemAssetData` (break `ItemDataStruct` _returnvalue))))))
    (:`RowNotFound`
      (`StaticMeshComponent.SetStaticMesh` (`self.ItemMesh`) null))))

(fn `LeaveStation`
  (`self.Open&Close`)
  (`parent.LeaveStation`))

(fn `OnPossessed`
  (`self.Open&Close`)
  (`parent.OnPossessed`))

(fn `OnUnPossessed`
  (`self.Open&Close`)
  (`parent.OnUnPossessed`))

(fn `TryStartMinigame`
  (returns (isMinigameStartSuccess :type Boolean))
  (bind _isminigamestartsuccess (`parent.TryStartMinigame`))
  (if _isminigamestartsuccess
    (`self.Open&Close`)
    (return _isminigamestartsuccess)))

(fn `UserConstructionScript`
  (`parent.UserConstructionScript`))