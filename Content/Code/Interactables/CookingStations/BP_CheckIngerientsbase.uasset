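; Base cooking-station interactable, apparently meant for ingredient checks, that opens its inventory container on the player's HUD when interacted with.
; Possession calls CheckIngredientsBaseFunction, whose entry does nothing as wired.
; Disconnected logic in that function would match inventory items against up to five Contents IDs and remove matched slots via ServerRemove.
; LookAt returns empty text.
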(event `self.ReceiveUnpossessed`
  (params (OldController :type "Controller Object Reference")))

(event `self.ReceivePossessed`
  (params (NewController :type "Controller Object Reference"))
  (`self.CheckIngredientsBaseFunction`))

(event `self.InteractWith`
  (params (PlayerCharacter :type "/Game/Code/Player/BP_Character Object Reference"))
  (bind _asbp_player_controller (cast `/Game/Code/Core/BP_PlayerController` (`GameplayStatics.GetPlayerController` 0)))
  (`/Game/Code/UI/UI_Inventory/W_PlayerHUD.ShowContainer` (`/Game/Code/Core/BP_PlayerController.HUD` _asbp_player_controller) (`self.BP_InventorySystem`)))

(fn `CheckIngredientsBaseFunction`
  (locals (ItemID :type Name) (DeleteItemOne :type Boolean) (DeleteItemTwo :type Boolean) (DeleteItemThree :type Boolean) (DeleteItemFour :type Boolean) (DeleteItemFive :type Boolean) (Length :type Integer :default 0) (ItemIndex :type Integer) (FirstItemIndex :type Integer) (SecondItemIndex :type Integer) (ThirdItemIndex :type Integer) (FourthItemIndex :type Integer) (FifthItemIndex :type Integer) (DeleteArray :type "Array of Boolean")))

(fn `LookAt`
  (returns (Message :type Text))
  (return ""))

(fn `UserConstructionScript`)