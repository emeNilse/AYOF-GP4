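; Base pickup item actor that the player interacts with to add its item and quantity to their inventory.
; OnInteract passes the item data component's ID to the pawn's BP_InventorySystem; success plays a triggered MetaSound, sends RespawnMessage to the owner and destroys the item.
; Failure logs and can start an inventory-full dialogue.
; LookAt returns the data table name and mesh, and OnInteract is meant for overriding.
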(event `/Game/Code/Core/Inventory/IInteractInterface.InteractWith`
  (params (PlayerCharacter :type "/Game/Code/Player/BP_Character Object Reference"))
  ; On Interact is called by the player controller on IA_Interact, so this event is also hooked up to OnInteract for backwards compatibility with some inventory functions
  ; override OnInteract function to do different things when the player presses the interact action and is in targeting range of the item
  (`self.OnInteract` null))

(event `self.ReceiveBeginPlay`)

(event `/Game/Code/Interactables/ItemIngridients/BPI_ItemSpawner.Respawn`
  (`self.RespawnBehavior`))

(fn `LookAt`
  (returns (Message :type Text) (SM :type "StaticMeshComponent Object Reference"))
  (bind (_itemid_datatable _itemid_rowname) (break `DataTableRowHandle` (`/Game/Code/Core/Inventory/BP_ItemDataComponent.ItemID` (`self.BP_ItemDataComponent`))))
  (bind _returnvalue (`|GetDataTableRow` _itemid_datatable _itemid_rowname)
    (:`then`
      (return (`.Name` (break `ItemTextData` (`.ItemTextData` (break `ItemDataStruct` _returnvalue)))) (`self.StaticMesh`)))))

(fn `OnInteract`
  (params (interactingPlayer :type "MyPlayerController Object Reference"))
  (bind _inventoryfull_dialogue (`self.InventoryFull Dialogue`))
  (bind _success (`self.SendSelfToInventory` interactingPlayer))
  (if _success
    ; successfully picked up, destroy and respawn pick up point prop
    (`self.PlayPickUpSound` (`self.MetasoundSource`))
    (`self.RespawnBehavior`)
    (`parent.OnInteract` (`local.interactingPlayer`))
    (else
      (`KismetSystemLibrary.PrintText` (`|FormatText` "{player} interacted with: {ownName}, and add to inventory failed" (`KismetSystemLibrary.GetDisplayName` interactingPlayer) (`KismetSystemLibrary.GetDisplayName` self)) true true (struct :`G` 0.66 :`B` 1.0 :`A` 1.0) 2.0 "BP_BaseItem_AddToInventoryFail")
      (if (`self.Show dialogue on inventory full`)
        (`DialogueEventComponent.StartDialogueEvent` (`self.BP_DialogueComponent`) _inventoryfull_dialogue false)
        (`KismetSystemLibrary.PrintString` (`KismetStringLibrary.Conv_NameToString` _inventoryfull_dialogue) true true (struct :`G` 0.66 :`B` 1.0 :`A` 1.0) 2.0 _inventoryfull_dialogue)))))

(fn `PlayPickUpSound`
  (params (Sound :type "SoundBase Object Reference"))
  (bind _returnvalue (`GameplayStatics.SpawnSoundAtLocation` Sound (`SceneComponent.K2_GetComponentLocation` (`self.DefaultSceneRoot`)) (struct) 1.0 1.0 0.0 null null))
  (`AudioParameterControllerInterface.SetTriggerParameter` _returnvalue "OnPickUp"))

(fn `RespawnBehavior`
  (message `/Game/Code/Interactables/ItemIngridients/BPI_ItemSpawner.Respawn` (`self.GetOwner`))
  (`self.K2_DestroyActor`)
  (`KismetSystemLibrary.PrintString` "BaseItemRespawnBPICalled"))

(fn `SendSelfToInventory`
  (params (InteractingPlayer :type "MyPlayerController Object Reference"))
  (returns (Success :type Boolean))
  (bind _bp_itemdatacomponent (`self.BP_ItemDataComponent`))
  (bind _characterpawn (`MyPlayerController.CharacterPawn` InteractingPlayer))
  (bind _returnvalue (`self.GetComponentByClass` _characterpawn "/Game/Code/Core/Inventory/BP_InventorySystem.BP_InventorySystem_C"))
  (bind (_itemid_datatable _itemid_rowname) (break `DataTableRowHandle` (`/Game/Code/Core/Inventory/BP_ItemDataComponent.ItemID` _bp_itemdatacomponent)))
  (`/Engine/EditorBlueprintResources/StandardMacros.IsValid` InteractingPlayer
    (:`Is Valid`
      (`/Engine/EditorBlueprintResources/StandardMacros.IsValid` _characterpawn
        (:`Is Valid`
          (`/Engine/EditorBlueprintResources/StandardMacros.IsValid` _returnvalue
            (:`Is Valid`
              (bind _success (`/Game/Code/Core/Inventory/BP_InventorySystem.AddToInventory` _returnvalue _itemid_rowname (`/Game/Code/Core/Inventory/BP_ItemDataComponent.Quantity` _bp_itemdatacomponent)))
              (return _success))))
        (:`Is Not Valid`
          (return false))))))

(fn `UserConstructionScript`)