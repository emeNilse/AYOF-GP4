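; BP_Spoon_MixingBowl is an interactable spoon actor that plays a one-shot animation with a mixing bowl sound.
; ReadyAnimation places the root at a hard-coded relative position, while TriggerAnimation plays the animation and spawns the sound.
; StopAnimation clears Active and rewinds the skeletal mesh to the start.
; Tick is empty, and an Active-gated sound-and-delay chain in the event graph is unconnected.
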(event `self.ReceiveTick`
  (params (DeltaSeconds :type "Float (single-precision)")))

(fn `ReadyAnimation`
  (bind _skeletalmesh (`self.SkeletalMesh`))
  (`SceneComponent.K2_SetRelativeTransform` (`self.DefaultSceneRoot`) (`KismetMathLibrary.MakeTransform` (-980.0 190.0 133.0)) false false)
  (`SkeletalMeshComponent.PlayAnimation` _skeletalmesh null false)
  (`SkeletalMeshComponent.Stop` _skeletalmesh))

(fn `StopAnimation`
  (bind _skeletalmesh (`self.SkeletalMesh`))
  (set `self.Active` false)
  (`SkeletalMeshComponent.Stop` _skeletalmesh)
  (`SkeletalMeshComponent.SetPosition` _skeletalmesh 0.0 false))

(fn `TriggerAnimation`
  (`SkeletalMeshComponent.PlayAnimation` (`self.SkeletalMesh`) "/Game/Art/1-Assets/Decorations/Animated/Spoon_Anim/SKM_Spoon_Interactable_Anim.SKM_Spoon_Interactable_Anim" false)
  (`GameplayStatics.SpawnSoundAtLocation` "/Game/Audio/MetaSounds/SFX/MS_MixingBowl.MS_MixingBowl" (0.0 0.0 0.0) (struct) 5.0 5.0 0.0 null null))

(fn `UserConstructionScript`)