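; Dialogue component that shows dialogue text and choices through a WB_DialogueMain widget.
; SendTextToUI updates the DialogueManager's shared on-screen widget or creates one, then sets the manager's text-based display timer, or stops it when choices await input.
; Without a manager, it keeps its own timer, but Tick passes a zero delta, so it never counts down.
; Selected choices are only printed for debugging before the widget is removed after a short delay.
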(event `self.ReceiveBeginPlay`)

(event `self.ReceiveTick`
  (params (DeltaSeconds :type "Float (single-precision)"))
  (bind _dialoguewidget (`self.DialogueWidget`))
  (`/Engine/EditorBlueprintResources/StandardMacros.IsValid` (`self.DialogueManager`)
    (:`Is Not Valid`
      (`/Engine/EditorBlueprintResources/StandardMacros.IsValid` _dialoguewidget
        (:`Is Valid`
          (if (and (`Widget.IsInViewport` _dialoguewidget) (not (`self.CurrentDialogueWaitsForInput`)))
            (`self.TickDisplayTimer` 0.0)))))))

(event `self.DialogueChoiceSelected`
  (params (value :type Byte) (choiceText :type "Text (by ref)") (bIsMinigameChoice :type Boolean))
  (`self.print choice result` value choiceText bIsMinigameChoice)
  (`KismetSystemLibrary.Delay` 0.2)
  (`Widget.RemoveFromParent` (`self.DialogueWidget`)))

(fn `IsDialogueOnScreen`
  (returns (isOnScreen :type Boolean))
  (bind _dialoguemanager (`self.DialogueManager`))
  (bind _centraldialoguewidget (`DialogueManagerComponent.CentralDialogueWidget` _dialoguemanager))
  (`/Engine/EditorBlueprintResources/StandardMacros.IsValid` _dialoguemanager
    (:`Is Valid`
      (`/Engine/EditorBlueprintResources/StandardMacros.IsValid` _centraldialoguewidget
        (:`Is Valid`
          (return (`Widget.IsInViewport` _centraldialoguewidget)))
        (:`Is Not Valid`
          (return false))))))

(fn `print choice result`
  (params (choiceValue :type Byte) (choiceText :type "Text (by ref)") (resultIsMinigame :type Boolean))
  (if resultIsMinigame
    ; choice as EValidMinigame
    (`KismetSystemLibrary.PrintString` (`KismetStringLibrary.Concat_StrStr` "Player chose: " (`KismetTextLibrary.Conv_TextToString` choiceText) ", value: " (`KismetStringLibrary.Conv_ByteToString` choiceValue)) true true (struct :`G` 0.66 :`B` 1.0 :`A` 1.0) 10.0)
    (else
      ; generic int value for choices
      (`KismetSystemLibrary.PrintString` (`KismetStringLibrary.Concat_StrStr` "Player chose: " (`KismetTextLibrary.Conv_TextToString` choiceText) ", value: " (`KismetStringLibrary.Conv_ByteToString` choiceValue)) true true (struct :`G` 0.66 :`B` 1.0 :`A` 1.0) 10.0))))

(fn `RemoveOldDialogue`
  (bind _asbp_ayof_game_mode (cast `/Game/Code/Core/GameModes/BP_AyofGameMode` (`GameplayStatics.GetGameMode`)))
  (bind _centraldialoguewidget (`/Game/Code/Core/GameModes/BP_AyofGameMode.CentralDialogueWidget` _asbp_ayof_game_mode))
  (`/Engine/EditorBlueprintResources/StandardMacros.IsValid` _centraldialoguewidget
    (:`Is Valid`
      (if (`Widget.IsInViewport` _centraldialoguewidget)
        (`Widget.RemoveFromParent` _centraldialoguewidget)))))

(fn `SendTextToUI`
  (params (dialogueData :type "DialogueDataStruct Structure (by ref)"))
  (locals (gameModeWithWidget :type "/Game/Code/Core/GameModes/BP_AyofGameMode Object Reference") (IsDialogueManagerValid :type Boolean :default false))
  (bind (_name _bcanrepeat _displaytext _bhaschoices _choices) (break `DialogueDataStruct` dialogueData))
  (bind (_name_2 _bcanrepeat_2 _displaytext_2 _bhaschoices_2) (break `DialogueDataStruct` dialogueData))
  (bind _dialoguemanager (`self.DialogueManager`))
  (set `local.IsDialogueManagerValid` (`KismetSystemLibrary.IsValid` (`self.DialogueManager`)))
  (`|ExecutionSequence`
    (:`then_0`
      (set `self.CurrentDialogueCanRepeat` _bcanrepeat_2))
    (:`then_1`
      (set `self.CurrentDialogueWaitsForInput` _bhaschoices_2))
    (:`then_2`
      (if (`self.IsDialogueOnScreen`)
        ; update existing widget
        (bind _aswb_dialogue_main (cast `/Game/Code/UI/Dialogue/WB_DialogueMain` (`DialogueManagerComponent.CentralDialogueWidget` (`self.DialogueManager`))))
        (`/Game/Code/UI/Dialogue/WB_DialogueMain.UpdateDialogueText` _aswb_dialogue_main _displaytext _choices _bhaschoices)
        (else
          ; create new widget
          (`parent.SendTextToUI` dialogueData)
          (bind _returnvalue (`|CreateWidget` "/Game/Code/UI/Dialogue/WB_DialogueMain.WB_DialogueMain_C" null _bhaschoices dialogueData self))
          (bind _output_get (set `self.DialogueWidget` _returnvalue))
          (if (`local.IsDialogueManagerValid`)
            (bind _output_get_2 (set `DialogueManagerComponent.CentralDialogueWidget` _output_get (`self.DialogueManager`)))
            (`UserWidget.AddToViewport` _output_get_2 0)))))
    (:`then_3`
      ; set duration for display timer
      (if (`self.CurrentDialogueWaitsForInput`)
        (if (`local.IsDialogueManagerValid`)
          (`DialogueManagerComponent.StopDisplayTimer` _dialoguemanager)
          (set `DialogueManagerComponent.CurrentDialogueWaitsForInput` true _dialoguemanager))
        (elif (`local.IsDialogueManagerValid`)
          (`DialogueManagerComponent.SetDisplayTimerByText` (`self.DialogueManager`) (`.DisplayText` (break `DialogueDataStruct` dialogueData)) 1.0)
          (else
            (set `self.DisplayTimer` 2.0)))))
    (:`then_4`
      (return))))

(fn `TickDisplayTimer`
  (params (B :type "Float (double-precision)"))
  (bind _output_get (set `self.DisplayTimer` (- (`self.DisplayTimer`) B)))
  (if (<= _output_get 0.0)
    (`|ExecutionSequence`
      (:`then_0`
        (`Widget.RemoveFromParent` (`self.DialogueWidget`)))
      (:`then_1`
        (`KismetSystemLibrary.PrintString` "Dialogue component removed the dialogue widget from timer")))))