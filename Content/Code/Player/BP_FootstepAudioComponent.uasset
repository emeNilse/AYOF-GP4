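; Player audio component that plays footstep sounds at a fixed interval while the move input is held.
; IA_Move starting plays an immediate step and starts a timer; completing it stops and resets the timer.
; Tick accumulates time and spawns MS_Footsteps attached to the owner's root whenever the step interval is reached.
; Cadence depends only on input and elapsed time, with no speed or ground check.
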(event `self.ReceiveBeginPlay`)

(event `self.ReceiveTick`
  (params (DeltaSeconds :type "Float (single-precision)"))
  (if (`self.bStepTimerRunning`)
    (bind _output_get (set `self.TimeSinceStep` (+ (`self.TimeSinceStep`) DeltaSeconds)))
    (`/Engine/EditorBlueprintResources/StandardMacros.CompareFloat` _output_get (`self.StepIntervalSeconds`)
      (:`>`
        _)
      (:`==`
        _))
    (`self.PlayFootstep`)
    (set `self.TimeSinceStep` 0.0)))

(event `EnhancedInput|/Game/Code/Input/Actions/IA_Move`
  (params (ActionValue :type "Vector2D Structure") (ElapsedSeconds :type "Float (double-precision)") (TriggeredSeconds :type "Float (double-precision)") (InputAction :type "InputAction Object Reference" :default "/Game/Code/Input/Actions/IA_Move.IA_Move"))
  (:`Started`
    (set `self.bStepTimerRunning` true)
    (`self.PlayFootstep`))
  (:`Completed`
    (set `self.bStepTimerRunning` false)
    (set `self.TimeSinceStep` 0.0)))

(fn `PlayFootstep`
  (`GameplayStatics.SpawnSoundAttached` "/Game/Audio/MetaSounds/SFX/MS_Footsteps.MS_Footsteps" (`Actor.RootComponent` (`self.GetOwner`)) "None" (0.0 0.0 0.0) (struct) "KeepRelativeOffset" true 1.0 1.0 0.0 null null)
  (set `self.TimeSinceStep` 0.0))