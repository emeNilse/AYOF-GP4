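; Mixing minigame actor where the player circles IA_JoystickL input to stir a bowl.
; Input angles convert to 0-360 degrees; increases add progress at device-specific rates and trigger the BP_Spoon_MixingBowl animation, while other readings add their angle to WrongRotation.
; Tick updates the widget's progress bar and, when full, plays a success sound, reports a three-tier quality based on WrongRotation, then destroys the actor.
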(event `self.ReceiveBeginPlay`
  (set `self.Widget` (`self.Widget_0`))
  (bind _returnvalue (`GameplayStatics.GetActorOfClass` "/Game/Code/Interactables/BP_Spoon_MixingBowl.BP_Spoon_MixingBowl_C"))
  (set `self.Spoon` _returnvalue)
  (`parent.ReceiveBeginPlay`))

(event `EnhancedInput|/Game/Code/Input/Actions/TaskInputs/IA_JoystickL`
  (params (ActionValue :type "Vector2D Structure") (ElapsedSeconds :type "Float (double-precision)") (TriggeredSeconds :type "Float (double-precision)") (InputAction :type "InputAction Object Reference" :default "/Game/Code/Input/Actions/TaskInputs/IA_JoystickL.IA_JoystickL"))
  (bind (_x _y) (`KismetMathLibrary.BreakVector2D` ActionValue))
  (bind (_x_2 _y_2) (`KismetMathLibrary.BreakVector2D` (`KismetMathLibrary.Normal2D` ActionValue)))
  (:`Triggered`
    (if (`self.UsingGamepad`)
      (set `self.Degrees` (`KismetMathLibrary.DegAtan2` _x _y))
      (else
        (set `self.Degrees` (`KismetMathLibrary.DegAtan2` _x_2 _y_2))))
    (if (< (`self.Degrees`) 0.0)
      (set `self.RotationValue` (+ (`self.Degrees`) 360.0))
      (else
        (set `self.RotationValue` (`self.Degrees`))))
    (if (< (`self.OldValue`) (`self.RotationValue`))
      (`self.Animation`)
      (if (`self.UsingGamepad`)
        (set `self.WinValue` (`KismetMathLibrary.FClamp` (+ (`self.CurrentValue`) 6.0) 0.0 100.0))
        (else
          (bind _output_get (set `self.WinValue` (`KismetMathLibrary.FClamp` (+ (`self.CurrentValue`) 0.2) 0.0 100.0)))))
      (set `self.CurrentValue` _output_get)
      (else
        (set `self.WrongRotation` (+ (`self.WrongRotation`) (`self.RotationValue`)))))
    (set `self.OldValue` (`self.RotationValue`))))

(event `self.ReceiveTick`
  (params (DeltaSeconds :type "Float (single-precision)"))
  (`ProgressBar.SetPercent` (`/Game/Code/Blueprints/Tasks/Minigames/W_Minigame4P2.ProgressBar2` (`self.Widget_0`)) (/ (`self.WinValue`) 100.0))
  (if (>= (`self.WinValue`) 100.0)
    (`GameplayStatics.SpawnSound2D` "/Game/Audio/SFX/Alpha/325112__fisch12345__success.325112__fisch12345__success" 0.8 1.0 0.0 null)
    (bind _quality (`self.DetermineQuality`))
    (`self.OnMinigameCompleted` _quality)
    (`self.K2_DestroyActor`)))

(fn `Animation`
  (bind _spoon (`self.Spoon`))
  (if (not (`SkeletalMeshComponent.IsPlaying` (`/Game/Code/Interactables/BP_Spoon_MixingBowl.SkeletalMesh` _spoon)))
    (`/Game/Code/Interactables/BP_Spoon_MixingBowl.TriggerAnimation` _spoon)))

(fn `DetermineQuality`
  (returns (Quality :type "Float (double-precision)"))
  (if (<= (`self.WrongRotation`) 600.0)
    (return 3.0)
    (elif (<= (`self.WrongRotation`) 2500.0)
      (return 2.0)
      (else
        (return 1.0)))))

(fn `UserConstructionScript`)