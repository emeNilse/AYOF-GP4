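; Button-mashing kneading minigame that fills a progress bar and reports a quality rating on completion.
; Each ButtonB press raises the progress, while Tick tracks elapsed time and uses a DoOnce with a short Delay to drain it periodically and refresh the widget.
; On reaching the maximum it plays a success sound, passes a three-tier rating based on completion time to the minigame-completed call, then destroys itself.
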(event `self.ReceiveBeginPlay`
  (set `self.Widget` (`self.Widget_0`))
  (`parent.ReceiveBeginPlay`))

(event `self.ReceiveTick`
  (params (DeltaSeconds :type "Float (single-precision)"))
  (set `self.Timer` (+ DeltaSeconds (`self.Timer`)))
  (`/Engine/EditorBlueprintResources/StandardMacros.DoOnce` false :!label _label
    (:`Completed`
      (set `self.ProgressBar` (`KismetMathLibrary.FClamp` (- (`self.ProgressBar`) 2.0) 0.0 100.0))
      (`KismetSystemLibrary.Delay` 0.1)
      (`ProgressBar.SetPercent` (`/Game/Code/Blueprints/Tasks/Minigames/W_Minigame1.ProgressBar1` (`self.Widget_0`)) (/ (`self.ProgressBar`) 100.0))
      (goto _label :!via `Reset`))))

(event `EnhancedInput|/Game/Code/Input/Actions/TaskInputs/IA_ButtonB`
  (params (ActionValue :type Boolean) (ElapsedSeconds :type "Float (double-precision)") (TriggeredSeconds :type "Float (double-precision)") (InputAction :type "InputAction Object Reference" :default "/Game/Code/Input/Actions/TaskInputs/IA_ButtonB.IA_ButtonB"))
  (:`Triggered`
    (set `self.ProgressBar` (`KismetMathLibrary.FClamp` (+ (`self.ProgressBar`) 10.0) 0.0 100.0))
    (if (== (`self.ProgressBar`) (`self.MaxValue`))
      (`GameplayStatics.SpawnSound2D` "/Game/Audio/SFX/Alpha/325112__fisch12345__success.325112__fisch12345__success" 0.8 1.0 0.0 null)
      (bind _quality (`self.DetermineQuality`))
      (`self.OnMinigameCompleted` _quality)
      (`self.K2_DestroyActor`))))

(fn `DetermineQuality`
  (returns (Quality :type "Float (double-precision)"))
  (if (<= (`self.Timer`) 3.9)
    (return 3.0)
    (elif (<= (`self.Timer`) 4.5)
      (return 2.0)
      (else
        (return 1.0)))))

(fn `UserConstructionScript`)