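; BP_MG_Stirring is a stirring timing minigame tied to a cooking pot spoon.
; Tick sweeps a looping radial slider at a frame-rate-dependent speed; left-button presses in the middle window raise progress and animate the spoon, while misses lower progress and count as wrong clicks.
; When progress fills, it plays a success sound, reports a quality tier based on wrong clicks through CallOnMinigameCompleted and destroys itself.
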(event `self.ReceiveBeginPlay`
  (set `self.Widget` (`self.Widget_0`))
  (`parent.ReceiveBeginPlay`)
  (bind _output_get (set `self.Progress` 0.0))
  (`ProgressBar.SetPercent` (`/Game/Code/Blueprints/Tasks/Minigames/W_Minigame5P2.ProgressBar2` (`self.Widget_0`)) _output_get)
  (bind _returnvalue (`GameplayStatics.GetActorOfClass` "/Game/Code/Interactables/BP_Spoon_CookingPot.BP_Spoon_CookingPot_C"))
  (set `self.Spoon` _returnvalue))

(event `EnhancedInput|/Game/Code/Input/Actions/TaskInputs/IA_ButtonL`
  (params (ActionValue :type Boolean) (ElapsedSeconds :type "Float (double-precision)") (TriggeredSeconds :type "Float (double-precision)") (InputAction :type "InputAction Object Reference" :default "/Game/Code/Input/Actions/TaskInputs/IA_ButtonL.IA_ButtonL"))
  (bind _slidervalue (`self.SliderValue`))
  (:`Triggered`
    (if (and (< _slidervalue 60.0) (> _slidervalue 40.0))
      (`self.Animation`)
      (bind _output_get (set `self.Progress` (`KismetMathLibrary.FClamp` (+ 30.0 (`self.Progress`)) 0.0 100.0)))
      (`ProgressBar.SetPercent` (`/Game/Code/Blueprints/Tasks/Minigames/W_Minigame5P2.ProgressBar2` (`self.Widget_0`)) (/ _output_get 100.0))
      (else
        (bind _output_get_2 (set `self.Progress` (`KismetMathLibrary.FClamp` (- (`self.Progress`) 15.0) 0.0 100.0)))
        (`ProgressBar.SetPercent` (`/Game/Code/Blueprints/Tasks/Minigames/W_Minigame5P2.ProgressBar2` (`self.Widget_0`)) (/ _output_get_2 100.0))
        (`/Engine/EditorBlueprintResources/StandardMacros.IncrementInt` (`self.WrongClicks`))))))

(event `self.ReceiveTick`
  (params (DeltaSeconds :type "Float (single-precision)"))
  (if (>= (`self.Progress`) 99.0)
    (`GameplayStatics.SpawnSound2D` "/Game/Audio/SFX/Alpha/325112__fisch12345__success.325112__fisch12345__success" 0.8 1.0 0.0 null)
    (bind _quality (`self.DetermineQuality`))
    (`self.OnMinigameCompleted` _quality)
    (`self.K2_DestroyActor`)
    (else
      (set `self.SliderValue` (`KismetMathLibrary.FClamp` (+ (`self.SliderValue`) 3.0) 0.0 100.0))
      (`RadialSlider.SetValue` (`/Game/Code/Blueprints/Tasks/Minigames/W_Minigame5P2.RadialSlider_0` (`self.Widget_0`)) (/ (`self.SliderValue`) 100.0))
      (if (<= 100.0 (`self.SliderValue`))
        (set `self.SliderValue` 0.0)))))

(fn `Animation`
  (bind _spoon (`self.Spoon`))
  (if (not (`SkeletalMeshComponent.IsPlaying` (`/Game/Code/Interactables/BP_Spoon_CookingPot.SkeletalMesh` _spoon)))
    (`/Game/Code/Interactables/BP_Spoon_CookingPot.TriggerAnimation` _spoon)))

(fn `DetermineQuality`
  (returns (Quality :type "Float (double-precision)"))
  (if (== (`self.WrongClicks`) 0)
    (return 3.0)
    (elif (== (`self.WrongClicks`) 1)
      (return 2.0)
      (else
        (return 1.0)))))

(fn `UserConstructionScript`)