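; Cutting minigame actor where the player times button presses to land a wrapping slider inside a randomly placed target zone.
; Tick moves the slider by a frame-rate-dependent step in the trigger-chosen direction and repositions the zone through border-slot padding after each press.
; Button B animates the knife and counts hits or misses, with hits filling a progress bar.
; Enough hits play a success sound, report miss-based quality and destroy the actor.
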(event `EnhancedInput|/Game/Code/Input/Actions/TaskInputs/IA_TriggerR`
  (params (ActionValue :type Boolean) (ElapsedSeconds :type "Float (double-precision)") (TriggeredSeconds :type "Float (double-precision)") (InputAction :type "InputAction Object Reference" :default "/Game/Code/Input/Actions/TaskInputs/IA_TriggerR.IA_TriggerR"))
  (:`Triggered`
    (set `self.MovesToRight` true)))

(event `EnhancedInput|/Game/Code/Input/Actions/TaskInputs/IA_TriggerL`
  (params (ActionValue :type Boolean) (ElapsedSeconds :type "Float (double-precision)") (TriggeredSeconds :type "Float (double-precision)") (InputAction :type "InputAction Object Reference" :default "/Game/Code/Input/Actions/TaskInputs/IA_TriggerL.IA_TriggerL"))
  (:`Triggered`
    (set `self.MovesToRight` false)))

(event `EnhancedInput|/Game/Code/Input/Actions/TaskInputs/IA_ButtonB`
  (params (ActionValue :type Boolean) (ElapsedSeconds :type "Float (double-precision)") (TriggeredSeconds :type "Float (double-precision)") (InputAction :type "InputAction Object Reference" :default "/Game/Code/Input/Actions/TaskInputs/IA_ButtonB.IA_ButtonB"))
  (bind _goalvalue (`self.GoalValue`))
  (bind _slidervalue (`self.SliderValue`))
  (:`Triggered`
    (set `self.ResetSlider` true)
    (`/Game/Code/Interactables/BP_Knife.TriggerAnimation` (`self.KnifeBP`))
    (if (and (>= _slidervalue (/ (- _goalvalue 30.0) 4.0)) (<= _slidervalue (/ (+ _goalvalue 30.0) 4.0)))
      (bind _result (`/Engine/EditorBlueprintResources/StandardMacros.IncrementInt` (`self.NumOfGoodClicks`))
        (:`  `
          (`ProgressBar.SetPercent` (`/Game/Code/Blueprints/Tasks/Minigames/W_Minigame3P1.ProgressBar2` (`self.Widget_0`)) (/ (`KismetMathLibrary.Conv_IntToDouble` _result) (`KismetMathLibrary.Conv_IntToDouble` (`self.NumOfClicksNeeded`))))))
      (else
        (bind _result_2 (`/Engine/EditorBlueprintResources/StandardMacros.IncrementInt` (`self.NumOfBadClicks`))
          (:`  `
            (set `self.NumOfBadClicks` _result_2)))))))

(event `self.ReceiveBeginPlay`
  (set `self.Widget` (`self.Widget_0`))
  (`parent.ReceiveBeginPlay`)
  (set `self.MovesToRight` true)
  (set `self.ResetSlider` true)
  (bind _returnvalue (`GameplayStatics.GetActorOfClass` "/Game/Code/Interactables/BP_Knife.BP_Knife_C"))
  (set `self.KnifeBP` _returnvalue))

(event `self.ReceiveTick`
  (params (DeltaSeconds :type "Float (single-precision)"))
  (bind _slidervalue (`self.SliderValue`))
  (bind _slidervalue_2 (`self.SliderValue`))
  (bind _goalvalue (`self.GoalValue`))
  (if (>= (`self.NumOfGoodClicks`) (`self.NumOfClicksNeeded`))
    (`GameplayStatics.SpawnSound2D` "/Game/Audio/SFX/Alpha/325112__fisch12345__success.325112__fisch12345__success" 0.8 1.0 0.0 null)
    (bind _quality (`self.DetermineQuality`))
    (`self.OnMinigameCompleted` _quality)
    (`self.K2_DestroyActor`)
    (elif (`self.ResetSlider`)
      (set `self.GoalValue` (`KismetMathLibrary.RandomFloatInRange` 35.0 365.0))
      (bind _asborder_slot (cast `BorderSlot` (`Widget.Slot` (`/Game/Code/Blueprints/Tasks/Minigames/W_Minigame3P1.ProgressBar1` (`self.Widget_0`)))))
      (`BorderSlot.SetPadding` _asborder_slot (make `Margin` (- _goalvalue 30.0) 6.0 (- 400.0 (+ _goalvalue 30.0)) 6.0))
      (set `self.ResetSlider` false)
      (elif (`self.MovesToRight`)
        (bind _output_get (set `self.SliderValue` (+ _slidervalue_2 2.0)))
        (`Slider.SetValue` (`/Game/Code/Blueprints/Tasks/Minigames/W_Minigame3P1.Slider1` (`self.Widget_0`)) (/ _output_get 100.0))
        (if (>= _slidervalue_2 100.0)
          (set `self.SliderValue` 0.0))
        (else
          (bind _output_get_2 (set `self.SliderValue` (+ _slidervalue -2.0)))
          (`Slider.SetValue` (`/Game/Code/Blueprints/Tasks/Minigames/W_Minigame3P1.Slider1` (`self.Widget_0`)) (/ _output_get_2 100.0))
          (if (<= _slidervalue 0.0)
            (set `self.SliderValue` 100.0)))))))

(fn `DetermineQuality`
  (returns (Quality :type "Float (double-precision)"))
  (if (== (`self.NumOfBadClicks`) 0)
    (return 3.0)
    (elif (== (`self.NumOfBadClicks`) 1)
      (return 2.0)
      (else
        (return 1.0)))))

(fn `UserConstructionScript`)