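; BP_MG is a minigame actor, apparently a base, that switches the player into task mode for as long as it is in play.
; On BeginPlay it adds its Widget to the viewport, swaps IMC_Default for IMC_Task and sets Game and UI input focused on that widget.
; On EndPlay it removes the widget and restores the default mapping context, but leaves the input mode as set.
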(event `self.ReceiveBeginPlay`
  (bind _returnvalue (`GameplayStatics.GetPlayerController` 0))
  (bind _returnvalue_2 (pcsubsystem `EnhancedInputLocalPlayerSubsystem` _returnvalue))
  (`UserWidget.AddToViewport` (`self.Widget`) 0)
  (`EnhancedInputSubsystemInterface.AddMappingContext` _returnvalue_2 "/Game/Code/Input/IMC_Task.IMC_Task" 0 (struct))
  (`EnhancedInputSubsystemInterface.RemoveMappingContext` _returnvalue_2 "/Game/Code/Input/IMC_Default.IMC_Default" (struct))
  (`WidgetBlueprintLibrary.SetInputMode_GameAndUIEx` _returnvalue (`self.Widget`)))

(event `self.ReceiveEndPlay`
  (params (EndPlayReason :type "EEndPlayReason Enum" :default "Destroyed"))
  (bind _returnvalue (pcsubsystem `EnhancedInputLocalPlayerSubsystem` (`GameplayStatics.GetPlayerController` 0)))
  (`Widget.RemoveFromParent` (`self.Widget`))
  (`EnhancedInputSubsystemInterface.AddMappingContext` _returnvalue "/Game/Code/Input/IMC_Default.IMC_Default" 0 (struct))
  (`EnhancedInputSubsystemInterface.RemoveMappingContext` _returnvalue "/Game/Code/Input/IMC_Task.IMC_Task" (struct)))

(fn `UserConstructionScript`)